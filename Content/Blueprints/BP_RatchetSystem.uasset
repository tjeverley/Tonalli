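; Ratchet and pulley actor that lifts a linked MovedObject according to the rotation of a capstan.
; BeginPlay stores the object's starting Z as BaseHeight.
; Each Tick derives a new Z from the current height, the absolute relative yaw of Spine and PulleyMultiplier, offset for the starting position.
; The result is clamped between BaseHeight and a yaw-dependent maximum, leaving X and Y unchanged.
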(event EventBeginPlay
  ;[0.15 0.15 0.15 0.5] Get Lifted Item Starting Position
  (Variables|Default|SetBaseHeight (.z (Transformation|GetActorLocation (Variables|Default|GetMovedObject)))))

(event Collision|EventActorBeginOverlap
  (params (OtherActor :type Actor%20Object%20Reference)))

(event EventTick
  (params (DeltaSeconds :type Float%20%28single-precision%29))
  (bind _spine (Variables|Default|GetSpine))
  (bind _movedobject (Variables|Default|GetMovedObject))
  (bind _baseheight (Variables|Default|GetBaseHeight))
  (bind _returnvalue (Transformation|GetActorLocation _movedobject))
  (bind _relativerotation (Variables|/Script/Engine.SceneComponent|GetRelativeRotation _spine))
  (bind _returnvalue_2 (Math|Float|Absolute(Float) (.yaw _relativerotation)))
  ;[0.15 0.15 0.15 0.5] Get Capstan Rotation Angle
  ;[0.15 0.15 0.15 0.5] Set Lifted Item Position
  (Transformation|SetActorLocation _movedobject (Math|Vector|MakeVector (.x _returnvalue) (.y _returnvalue) (Math|Float|Clamp(Float) (- (* (+ (.z _returnvalue) _returnvalue_2) (Variables|Default|GetPulleyMultiplier)) (* (Variables|Default|GetBaseHeight) (- (Variables|Default|GetPulleyMultiplier) 1.0))) _baseheight (* (+ _baseheight _returnvalue_2) (Variables|Default|GetPulleyMultiplier)))) false false))

(fn ConstructionScript)