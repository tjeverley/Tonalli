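; Checkpoint trigger actor that autosaves the game when the player character enters its trigger volume.
; BeginPlay caches the player as BP_ThirdPersonCharacter, and the Trigger overlap event ignores any other actor.
; On a player overlap it calls Autosave on BP_GameInstance, fetching and caching that reference lazily on first use.
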(event OnComponentBeginOverlap(Trigger)
  (params (OverlappedComponent :type Primitive%20Component%20Object%20Reference) (OtherActor :type Actor%20Object%20Reference) (OtherComp :type Primitive%20Component%20Object%20Reference) (OtherBodyIndex :type Integer) (bFromSweep :type Boolean) (SweepResult :type Hit%20Result%20Structure%20%28by%20ref%29))
  (if (== OtherActor (Variables|Default|GetPlayerRef))
    (Utilities|IsValid (Variables|Default|GetGameInstRef)
      (:Is%20Valid
        _)
      (:Is%20Not%20Valid
        (bind _asbp_game_instance (Utilities|Casting|CastToBP_GameInstance (Game|GetGameInstance)))
        (bind _output_get (Variables|Default|SetGameInstRef _asbp_game_instance))))
    (Default|Autosave _output_get)))

(event EventBeginPlay
  (Utilities|IsValid (Variables|Default|GetPlayerRef)
    (:Is%20Not%20Valid
      (bind _asbp_third_person_character (Utilities|Casting|CastToBP_ThirdPersonCharacter (Game|GetPlayerCharacter 0)))
      (Variables|Default|SetPlayerRef _asbp_third_person_character))))

(event Collision|EventActorBeginOverlap
  (params (OtherActor :type Actor%20Object%20Reference)))

(event EventTick
  (params (DeltaSeconds :type Float%20%28single-precision%29)))

(fn ConstructionScript)