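; BP_UpgradeShard is a spinning pickup that opens the player's upgrade menu.
; An InteractionDetector overlap caches the BP_ThirdPersonCharacter reference and toggles both the prompt widget and CanInteract.
; Tick rotates the shard, turns the prompt toward the camera and polls the player's Interaction flag.
; On interaction it adds the player's UpgradeRef widget to the viewport, destroys itself, pauses the game and enables mouse-driven UI input.
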(event OnComponentBeginOverlap(InteractionDetector)
  (params (OverlappedComponent :type Primitive%20Component%20Object%20Reference) (OtherActor :type Actor%20Object%20Reference) (OtherComp :type Primitive%20Component%20Object%20Reference) (OtherBodyIndex :type Integer) (bFromSweep :type Boolean) (SweepResult :type Hit%20Result%20Structure%20%28by%20ref%29))
  ;[0.15 0.15 0.15 0.5] Display/Hide UI
  (Utilities|IsValid (Variables|Default|GetPlayerRef)
    (:Is%20Valid
      _)
    (:Is%20Not%20Valid
      (bind _asbp_third_person_character (Utilities|Casting|CastToBP_ThirdPersonCharacter OtherActor))
      (Variables|Default|SetPlayerRef _asbp_third_person_character)))
  (Rendering|SetVisibility (Variables|Default|GetPickUpMessage) true false)
  (Variables|Default|SetbCanInteract true))

(event OnComponentEndOverlap(InteractionDetector)
  (params (OverlappedComponent :type Primitive%20Component%20Object%20Reference) (OtherActor :type Actor%20Object%20Reference) (OtherComp :type Primitive%20Component%20Object%20Reference) (OtherBodyIndex :type Integer))
  ;[0.15 0.15 0.15 0.5] Display/Hide UI
  (Utilities|IsValid (Variables|Default|GetPlayerRef)
    (:Is%20Valid
      _)
    (:Is%20Not%20Valid
      (bind _asbp_third_person_character (Utilities|Casting|CastToBP_ThirdPersonCharacter OtherActor))
      (Variables|Default|SetPlayerRef _asbp_third_person_character)))
  (Rendering|SetVisibility (Variables|Default|GetPickUpMessage) false false)
  (Variables|Default|SetbCanInteract false))

(event EventBeginPlay
  ;[0.15 0.15 0.15 0.5] Default Values
  (Rendering|SetVisibility (Variables|Default|GetPickUpMessage) false false))

(event Collision|EventActorBeginOverlap
  (params (OtherActor :type Actor%20Object%20Reference)))

(event EventTick
  (params (DeltaSeconds :type Float%20%28single-precision%29))
  ;[0.15 0.15 0.15 0.5] Item Spin
  (CallFunction|Spin)
  (CallFunction|WidgetFacePlayer)
  (Utilities|IsValid (Variables|Default|GetPlayerRef)
    (:Is%20Valid
      _)
    (:Is%20Not%20Valid
      (bind _asbp_third_person_character (Utilities|Casting|CastToBP_ThirdPersonCharacter (Variables|Default|GetPlayerRef)))
      (bind _output_get (Variables|Default|SetPlayerRef _asbp_third_person_character))))
  (if (and (Variables|/Game/ThirdPerson/Blueprints/BP_ThirdPersonCharacter.BP_ThirdPersonCharacter_C|GetbInteraction _output_get) (Variables|Default|GetbCanInteract))
    (CallFunction|UpgradeMenu)))

(fn ConstructionScript)

(fn Spin
  (bind _shardbody (Variables|Default|GetShardBody))
  (Transformation|SetRelativeRotation _shardbody (Math|Rotator|MakeRotator 0.0 0.0 (+ (.yaw (Variables|/Script/Engine.SceneComponent|GetRelativeRotation _shardbody)) (Variables|Default|GetSpinRate))) false false)
  (return))

(fn WidgetFacePlayer
  ;[0.15 0.15 0.15 0.5] Orient UI to Face Player
  (Transformation|SetWorldRotation (Variables|Default|GetPickUpMessage) (Math|Rotator|FindLookatRotation (Transformation|GetWorldLocation (Variables|Default|GetPickUpMessage)) (Transformation|GetWorldLocation (Variables|/Script/Engine.PlayerCameraManager|GetTransformComponent (Game|GetPlayerCameraManager 0)))) false false)
  (return))

(fn UpgradeMenu
  (bind _returnvalue (Game|GetPlayerController 0))
  (bind _playerref (Variables|Default|GetPlayerRef))
  (bind _upgrade_ref (Variables|/Game/ThirdPerson/Blueprints/BP_ThirdPersonCharacter.BP_ThirdPersonCharacter_C|GetUpgrade%20Ref _playerref))
  (UserInterface|Viewport|AddtoViewport _upgrade_ref 0)
  (Actor|DestroyActor)
  (Game|SetGamePaused true)
  (Variables|/Script/Engine.PlayerController|SetbShowMouseCursor _returnvalue true)
  (Input|SetInputModeGameandUI _returnvalue _upgrade_ref "DoNotLock" true false)
  (return))