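; BP_FoundMessage is a pickup message that the player can read through the character's dialogue system.
; Overlapping InteractionDetector shows a prompt widget turned once toward the camera, enables interaction and sets the player's Dialogue flag; leaving reverses this.
; Tick polls the player's interaction flags and copies the message name and contents into DialogueRef.
; If ShowTutorial is set, overlap also triggers a BPTutorial popup until it is marked dismissed.
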(event OnComponentBeginOverlap(InteractionDetector)
  (params (OverlappedComponent :type Primitive%20Component%20Object%20Reference) (OtherActor :type Actor%20Object%20Reference) (OtherComp :type Primitive%20Component%20Object%20Reference) (OtherBodyIndex :type Integer) (bFromSweep :type Boolean) (SweepResult :type Hit%20Result%20Structure%20%28by%20ref%29))
  ;[0.15 0.15 0.15 0.5] Display/Hide UI
  (Utilities|IsValid (Variables|Default|GetPlayerRef)
    (:Is%20Valid
      _)
    (:Is%20Not%20Valid
      (bind _asbp_third_person_character (Utilities|Casting|CastToBP_ThirdPersonCharacter (Game|GetPlayerCharacter 0)))
      (bind _output_get (Variables|Default|SetPlayerRef _asbp_third_person_character))))
  (if (== OtherActor (Variables|Default|GetPlayerRef))
    (CallFunction|WidgetFacePlayer)
    (Rendering|SetVisibility (Variables|Default|GetInteractionMessage) true false)
    (Variables|Default|SetbCanInteract true)
    (Variables|/Game/ThirdPerson/Blueprints/BP_ThirdPersonCharacter.BP_ThirdPersonCharacter_C|SetbDialogue _output_get true)
    (if (Variables|Default|GetbShowTutorial)
      (CallFunction|Tutorial))))

(event OnComponentEndOverlap(InteractionDetector)
  (params (OverlappedComponent :type Primitive%20Component%20Object%20Reference) (OtherActor :type Actor%20Object%20Reference) (OtherComp :type Primitive%20Component%20Object%20Reference) (OtherBodyIndex :type Integer))
  ;[0.15 0.15 0.15 0.5] Display/Hide UI
  (Utilities|IsValid (Variables|Default|GetPlayerRef)
    (:Is%20Valid
      _)
    (:Is%20Not%20Valid
      (bind _asbp_third_person_character (Utilities|Casting|CastToBP_ThirdPersonCharacter (Game|GetPlayerCharacter 0)))
      (bind _output_get (Variables|Default|SetPlayerRef _asbp_third_person_character))))
  (if (== OtherActor (Variables|Default|GetPlayerRef))
    (Rendering|SetVisibility (Variables|Default|GetInteractionMessage) false false)
    (Variables|Default|SetbCanInteract false)
    (Variables|/Game/ThirdPerson/Blueprints/BP_ThirdPersonCharacter.BP_ThirdPersonCharacter_C|SetbDialogue _output_get false)))

(event EventBeginPlay
  ;[0.15 0.15 0.15 0.5] Default Values
  (Rendering|SetVisibility (Variables|Default|GetInteractionMessage) false false))

(event Collision|EventActorBeginOverlap
  (params (OtherActor :type Actor%20Object%20Reference)))

(event EventTick
  (params (DeltaSeconds :type Float%20%28single-precision%29))
  (Utilities|IsValid (Variables|Default|GetPlayerRef)
    (:Is%20Valid
      _)
    (:Is%20Not%20Valid
      (bind _asbp_third_person_character (Utilities|Casting|CastToBP_ThirdPersonCharacter (Variables|Default|GetPlayerRef)))
      (bind _output_get (Variables|Default|SetPlayerRef _asbp_third_person_character))))
  (if (Math|Boolean|ANDBoolean (Variables|/Game/ThirdPerson/Blueprints/BP_ThirdPersonCharacter.BP_ThirdPersonCharacter_C|GetbInteraction _output_get) (Variables|/Game/ThirdPerson/Blueprints/BP_ThirdPersonCharacter.BP_ThirdPersonCharacter_C|GetbDialogue _output_get) (Variables|Default|GetbCanInteract))
    (CallFunction|OpenMessage)))

(fn ConstructionScript)

(fn WidgetFacePlayer
  ;[0.15 0.15 0.15 0.5] Orient UI To Face Player
  (Transformation|SetWorldRotation (Variables|Default|GetInteractionMessage) (Math|Rotator|FindLookatRotation (Transformation|GetWorldLocation (Variables|Default|GetInteractionMessage)) (Transformation|GetWorldLocation (Variables|/Script/Engine.PlayerCameraManager|GetTransformComponent (Game|GetPlayerCameraManager 0)))) false false)
  (return))

(fn OpenMessage
  (bind _playerref (Variables|Default|GetPlayerRef))
  (bind _dialogueref (Variables|/Game/ThirdPerson/Blueprints/BP_ThirdPersonCharacter.BP_ThirdPersonCharacter_C|GetDialogueRef _playerref))
  (Variables|/Game/UI/HUD/WBP_DialogueBox.WBP_DialogueBox_C|SetNameVar _dialogueref (Variables|Default|GetMessageName))
  (Variables|/Game/UI/HUD/WBP_DialogueBox.WBP_DialogueBox_C|SetDialogueVar _dialogueref (Variables|Default|GetMessageContents))
  (return))

(fn Tutorial
  (bind _bp_tutorial (Variables|Default|GetBP_Tutorial))
  (Utilities|IsValid (Variables|Default|GetPlayerRef)
    (:Is%20Valid
      _)
    (:Is%20Not%20Valid
      (bind _asbp_third_person_character (Utilities|Casting|CastToBP_ThirdPersonCharacter (Game|GetPlayerCharacter 0)))
      (bind _output_get (Variables|Default|SetPlayerRef _asbp_third_person_character))))
  (Variables|/Game/ThirdPerson/Blueprints/BP_ThirdPersonCharacter.BP_ThirdPersonCharacter_C|SetbDialogue _output_get true)
  (if (Variables|/Game/Blueprints/Tutorials/BP_Tutorial.BP_Tutorial_C|GetbDismissed _bp_tutorial)
    (return)
    (else
      (Default|ShowTutorial _bp_tutorial)
      (Default|DialogueBox (Variables|Default|GetPlayerRef))
      (Variables|/Game/Blueprints/Tutorials/BP_Tutorial.BP_Tutorial_C|SetbDismissed (Variables|Default|GetBP_Tutorial) true)
      (return))))