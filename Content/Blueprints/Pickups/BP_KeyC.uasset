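; BP_KeyC is a key pickup that adds one KeyC to the player's inventory.
; Overlapping InteractionDetector shows the pickup prompt, turns it once toward the camera and enables interaction; leaving hides and disables it.
; Tick polls the player's Interaction flag while enabled, then plays a sound, increments the count, autosaves through BP_GameInstance as a checkpoint and destroys the actor.
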(event OnComponentBeginOverlap(InteractionDetector)
  (params (OverlappedComponent :type Primitive%20Component%20Object%20Reference) (OtherActor :type Actor%20Object%20Reference) (OtherComp :type Primitive%20Component%20Object%20Reference) (OtherBodyIndex :type Integer) (bFromSweep :type Boolean) (SweepResult :type Hit%20Result%20Structure%20%28by%20ref%29))
  ;[0.15 0.15 0.15 0.5] Display/Hide UI
  (if (== OtherActor (Variables|Default|GetPlayerRef))
    (CallFunction|WidgetFacePlayer)
    (Rendering|SetVisibility (Variables|Default|GetPickUpMessage) true false)
    (Variables|Default|SetbCanInteract true)))

(event OnComponentEndOverlap(InteractionDetector)
  (params (OverlappedComponent :type Primitive%20Component%20Object%20Reference) (OtherActor :type Actor%20Object%20Reference) (OtherComp :type Primitive%20Component%20Object%20Reference) (OtherBodyIndex :type Integer))
  ;[0.15 0.15 0.15 0.5] Display/Hide UI
  (if (== OtherActor (Variables|Default|GetPlayerRef))
    (Rendering|SetVisibility (Variables|Default|GetPickUpMessage) false false)
    (Variables|Default|SetbCanInteract false)))

(event EventBeginPlay
  (Utilities|IsValid (Variables|Default|GetPlayerRef)
    (:Is%20Valid
      _)
    (:Is%20Not%20Valid
      (bind _asbp_third_person_character (Utilities|Casting|CastToBP_ThirdPersonCharacter (Game|GetPlayerCharacter 0)))
      (Variables|Default|SetPlayerRef _asbp_third_person_character)))
  ;[0.15 0.15 0.15 0.5] Default Values
  (Rendering|SetVisibility (Variables|Default|GetPickUpMessage) false false))

(event Collision|EventActorBeginOverlap
  (params (OtherActor :type Actor%20Object%20Reference)))

(event EventTick
  (params (DeltaSeconds :type Float%20%28single-precision%29))
  ;[0.15 0.15 0.15 0.5] Pick Up Key
  (Utilities|IsValid (Variables|Default|GetPlayerRef)
    (:Is%20Valid
      _)
    (:Is%20Not%20Valid
      (bind _asbp_third_person_character (Utilities|Casting|CastToBP_ThirdPersonCharacter (Game|GetPlayerCharacter 0)))
      (bind _output_get (Variables|Default|SetPlayerRef _asbp_third_person_character))))
  (if (and (Variables|/Game/ThirdPerson/Blueprints/BP_ThirdPersonCharacter.BP_ThirdPersonCharacter_C|GetbInteraction _output_get) (Variables|Default|GetbCanInteract))
    (Audio|PlaySound2D "/Game/Audio/SoundEffects/Character/Key_Item_collected.Key_Item_collected" 1.0 1.0 0.0 0 0)
    (CallFunction|AddKeytoInventory)))

(fn ConstructionScript)

(fn AddKeytoInventory
  (bind _playerref (Variables|Default|GetPlayerRef))
  (bind _playerinventory (Variables|/Game/ThirdPerson/Blueprints/BP_ThirdPersonCharacter.BP_ThirdPersonCharacter_C|GetPlayerInventory _playerref))
  ;[0.15 0.15 0.15 0.5] Increment Number of Keys in Inventory
  (Variables|/Game/ThirdPerson/Blueprints/BP_Inventory.BP_Inventory_C|SetKeyC _playerinventory (+ (Variables|/Game/ThirdPerson/Blueprints/BP_Inventory.BP_Inventory_C|GetKeyC _playerinventory) 1))
  ;[0.15 0.15 0.15 0.5] Checkpoint
  (Utilities|IsValid (Variables|Default|GetInstRef)
    (:Is%20Valid
      _)
    (:Is%20Not%20Valid
      (bind _asbp_game_instance (Utilities|Casting|CastToBP_GameInstance (Game|GetGameInstance)))
      (bind _output_get (Variables|Default|SetInstRef _asbp_game_instance))))
  (Default|Autosave _output_get)
  ;[0.15 0.15 0.15 0.5] Remove Collected Key From Map
  (Actor|DestroyActor self)
  (return))

(fn WidgetFacePlayer
  ;[0.15 0.15 0.15 0.5] Orient UI to Face Player
  (Transformation|SetWorldRotation (Variables|Default|GetPickUpMessage) (Math|Rotator|FindLookatRotation (Transformation|GetWorldLocation (Variables|Default|GetPickUpMessage)) (Transformation|GetWorldLocation (Variables|/Script/Engine.PlayerCameraManager|GetTransformComponent (Game|GetPlayerCameraManager 0)))) false false)
  (return))