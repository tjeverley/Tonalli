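; Heart pickup that appears once every tracked golem enemy is dead and adds a Stone Heart to the player's inventory.
; Tick removes enemies at zero health from the Enemies array and, when it is empty, reveals the heart with collision.
; Overlapping the detector while the heart is visible shows a prompt turned toward the camera and enables pickup.
; The player's Interaction flag, polled on Tick, collects the heart and destroys the actor.
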(event OnComponentBeginOverlap(HeartPickUpDetector)
  (params (OverlappedComponent :type Primitive%20Component%20Object%20Reference) (OtherActor :type Actor%20Object%20Reference) (OtherComp :type Primitive%20Component%20Object%20Reference) (OtherBodyIndex :type Integer) (bFromSweep :type Boolean) (SweepResult :type Hit%20Result%20Structure%20%28by%20ref%29))
  ;[0.15 0.15 0.15 0.5] Display/Hide UI
  (Utilities|IsValid (Variables|Default|GetPlayerRef)
    (:Is%20Valid
      _)
    (:Is%20Not%20Valid
      (bind _asbp_third_person_character (Utilities|Casting|CastToBP_ThirdPersonCharacter OtherActor))
      (Variables|Default|SetPlayerRef _asbp_third_person_character)))
  (if (Rendering|IsVisible (Variables|Default|GetHeart))
    (CallFunction|WidgetFacePlayer)
    (Rendering|SetVisibility (Variables|Default|GetPickUpMessage) true false)
    (Variables|Default|SetbCanPickUp true)))

(event OnComponentEndOverlap(HeartPickUpDetector)
  (params (OverlappedComponent :type Primitive%20Component%20Object%20Reference) (OtherActor :type Actor%20Object%20Reference) (OtherComp :type Primitive%20Component%20Object%20Reference) (OtherBodyIndex :type Integer))
  ;[0.15 0.15 0.15 0.5] Display/Hide UI
  (Utilities|IsValid (Variables|Default|GetPlayerRef)
    (:Is%20Valid
      _)
    (:Is%20Not%20Valid
      (bind _asbp_third_person_character (Utilities|Casting|CastToBP_ThirdPersonCharacter OtherActor))
      (Variables|Default|SetPlayerRef _asbp_third_person_character)))
  (if (Rendering|IsVisible (Variables|Default|GetHeart))
    (Rendering|SetVisibility (Variables|Default|GetPickUpMessage) false false)
    (Variables|Default|SetbCanPickUp false)))

(event EventBeginPlay)

(event Collision|EventActorBeginOverlap
  (params (OtherActor :type Actor%20Object%20Reference)))

(event EventTick
  (params (DeltaSeconds :type Float%20%28single-precision%29))
  ;[0.15 0.15 0.15 0.5] Track Remaining Enemies
  (CallFunction|TrackRemainingEnemies)
  ;[0.15 0.15 0.15 0.5] Pick Up Heart
  (Utilities|IsValid (Variables|Default|GetPlayerRef)
    (:Is%20Valid
      _)
    (:Is%20Not%20Valid
      (bind _asbp_third_person_character (Utilities|Casting|CastToBP_ThirdPersonCharacter (Variables|Default|GetPlayerRef)))
      (bind _output_get (Variables|Default|SetPlayerRef _asbp_third_person_character))))
  (if (and (Variables|/Game/ThirdPerson/Blueprints/BP_ThirdPersonCharacter.BP_ThirdPersonCharacter_C|GetbInteraction _output_get) (Variables|Default|GetbCanPickUp))
    (Variables|/Game/ThirdPerson/Blueprints/BP_Inventory.BP_Inventory_C|SetStoneHearts (Variables|/Game/ThirdPerson/Blueprints/BP_ThirdPersonCharacter.BP_ThirdPersonCharacter_C|GetPlayerInventory _output_get) (+ (Variables|/Game/ThirdPerson/Blueprints/BP_Inventory.BP_Inventory_C|GetStoneHearts (Variables|/Game/ThirdPerson/Blueprints/BP_ThirdPersonCharacter.BP_ThirdPersonCharacter_C|GetPlayerInventory _output_get)) 1))
    (Actor|DestroyActor)))

(fn ConstructionScript)

(fn RemovefromList
  (params (EnemyList :type Array%20of%20Pawn%20Object%20References) (ArrayIndex :type Integer))
  (Utilities|Array|RemoveItem EnemyList (Utilities|Array|Get(acopy) EnemyList ArrayIndex))
  (return))

(fn DropHeart
  (bind _heart (Variables|Default|GetHeart))
  (Collision|SetCollisionEnabled _heart "QueryAndPhysics")
  (Rendering|SetVisibility _heart true false)
  (Components|Tick|SetComponentTickEnabled _heart true)
  (return))

(fn TrackRemainingEnemies
  (bind _enemies (Variables|Default|GetEnemies))
  (bind _returnvalue (Utilities|Array|Length _enemies))
  ;[0.15 0.15 0.15 0.5] After All Enemies Dead
  (if (== _returnvalue 0)
    ;[0.15 0.15 0.15 0.5] Drop Loot
    (CallFunction|DropHeart)
    (else
      ;[0.15 0.15 0.15 0.5] Check Enemies in Array
      (for _index (range 0 (- _returnvalue 1))
        ;[0.15 0.15 0.15 0.5] Check Enemy HP
        (if (<= (Variables|/Game/Characters/Enemies/StoneMeleeGolom/Blueprints/BP_StoneMeleeGolom.BP_StoneMeleeGolom_C|GetGolemHealth (Utilities|Array|Get(acopy) (Variables|Default|GetEnemies) _index)) 0.0)
          ;[0.15 0.15 0.15 0.5] Remove From Array Upon Death
          (CallFunction|RemovefromList (Variables|Default|GetEnemies) _index))
        (return))))
  (return))

(fn WidgetFacePlayer
  ;[0.15 0.15 0.15 0.5] Orient UI to Face Player
  (Transformation|SetWorldRotation (Variables|Default|GetPickUpMessage) (Math|Rotator|FindLookatRotation (Transformation|GetWorldLocation (Variables|Default|GetPickUpMessage)) (Transformation|GetWorldLocation (Variables|/Script/Engine.PlayerCameraManager|GetTransformComponent (Game|GetPlayerCameraManager 0)))) false false)
  (return))