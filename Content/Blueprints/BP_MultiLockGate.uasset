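; Two-slot gate that slides its doors apart once the player has placed both Key A and Key B.
; Slot overlaps cache the player, check inventory, show a has-key or missing-key prompt, and enable interaction.
; Tick polls the player's Interaction flag; UseKeyA/B decrement inventory, reveal the key and mark it unlocked, then the key animates into its slot.
; With both unlocked, Tick plays a delayed timeline that moves both doors.
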(event OnComponentBeginOverlap(KeyASlot)
  (params (OverlappedComponent :type Primitive%20Component%20Object%20Reference) (OtherActor :type Actor%20Object%20Reference) (OtherComp :type Primitive%20Component%20Object%20Reference) (OtherBodyIndex :type Integer) (bFromSweep :type Boolean) (SweepResult :type Hit%20Result%20Structure%20%28by%20ref%29))
  (bind _keya (Variables|Default|GetKeyA))
  (bind _returnvalue (Rendering|IsVisible _keya))
  (bind _returnvalue_2 (not _returnvalue))
  ;[0.15 0.15 0.15 0.5] Slot A UI
  ;;[0.15 0.15 0.15 0.5] Display Key Slot A UI
  (Utilities|IsValid (Variables|Default|GetPlayerRef)
    (:Is%20Valid
      _)
    (:Is%20Not%20Valid
      (bind _asbp_third_person_character (Utilities|Casting|CastToBP_ThirdPersonCharacter OtherActor))
      (bind _output_get (Variables|Default|SetPlayerRef _asbp_third_person_character))))
  ;;;[0.15 0.15 0.15 0.5] Check For Keys
  (if (> (Variables|/Game/ThirdPerson/Blueprints/BP_Inventory.BP_Inventory_C|GetKeyA (Variables|/Game/ThirdPerson/Blueprints/BP_ThirdPersonCharacter.BP_ThirdPersonCharacter_C|GetPlayerInventory _output_get)) 0)
    (Rendering|SetVisibility (Variables|Default|GetHasKeyA_Message) _returnvalue_2 false)
    (Variables|Default|SetbCanInteract_A _returnvalue_2)
    (else
      (Rendering|SetVisibility (Variables|Default|GetMissingKeyA_Message) _returnvalue_2 false))))

(event OnComponentBeginOverlap(KeyBSlot)
  (params (OverlappedComponent :type Primitive%20Component%20Object%20Reference) (OtherActor :type Actor%20Object%20Reference) (OtherComp :type Primitive%20Component%20Object%20Reference) (OtherBodyIndex :type Integer) (bFromSweep :type Boolean) (SweepResult :type Hit%20Result%20Structure%20%28by%20ref%29))
  (bind _keyb (Variables|Default|GetKeyB))
  (bind _returnvalue (Rendering|IsVisible _keyb))
  (bind _returnvalue_2 (not _returnvalue))
  ;[0.15 0.15 0.15 0.5] Slot B UI
  ;;[0.15 0.15 0.15 0.5] Display Key Slot B UI
  (Utilities|IsValid (Variables|Default|GetPlayerRef)
    (:Is%20Valid
      _)
    (:Is%20Not%20Valid
      (bind _asbp_third_person_character (Utilities|Casting|CastToBP_ThirdPersonCharacter OtherActor))
      (bind _output_get (Variables|Default|SetPlayerRef _asbp_third_person_character))))
  ;;;[0.15 0.15 0.15 0.5] Check For Keys
  (if (> (Variables|/Game/ThirdPerson/Blueprints/BP_Inventory.BP_Inventory_C|GetKeyB (Variables|/Game/ThirdPerson/Blueprints/BP_ThirdPersonCharacter.BP_ThirdPersonCharacter_C|GetPlayerInventory _output_get)) 0)
    (Rendering|SetVisibility (Variables|Default|GetHasKeyB_Message) _returnvalue_2 false)
    (Variables|Default|SetbCanInteract_B _returnvalue_2)
    (else
      (Rendering|SetVisibility (Variables|Default|GetMissingKeyB_Message) _returnvalue_2 false))))

(event OnComponentEndOverlap(KeyASlot)
  (params (OverlappedComponent :type Primitive%20Component%20Object%20Reference) (OtherActor :type Actor%20Object%20Reference) (OtherComp :type Primitive%20Component%20Object%20Reference) (OtherBodyIndex :type Integer))
  ;[0.15 0.15 0.15 0.5] Slot A UI
  ;;[0.15 0.15 0.15 0.5] Hide Key Slot A UI
  (Utilities|IsValid (Variables|Default|GetPlayerRef)
    (:Is%20Valid
      _)
    (:Is%20Not%20Valid
      (bind _asbp_third_person_character (Utilities|Casting|CastToBP_ThirdPersonCharacter OtherActor))
      (Variables|Default|SetPlayerRef _asbp_third_person_character)))
  (Rendering|SetVisibility (Variables|Default|GetHasKeyA_Message) false false)
  (Rendering|SetVisibility (Variables|Default|GetMissingKeyA_Message) false false)
  (Variables|Default|SetbCanInteract_A false))

(event OnComponentEndOverlap(KeyBSlot)
  (params (OverlappedComponent :type Primitive%20Component%20Object%20Reference) (OtherActor :type Actor%20Object%20Reference) (OtherComp :type Primitive%20Component%20Object%20Reference) (OtherBodyIndex :type Integer))
  ;[0.15 0.15 0.15 0.5] Slot B UI
  ;;[0.15 0.15 0.15 0.5] Hide Key Slot B UI
  (Utilities|IsValid (Variables|Default|GetPlayerRef)
    (:Is%20Valid
      _)
    (:Is%20Not%20Valid
      (bind _asbp_third_person_character (Utilities|Casting|CastToBP_ThirdPersonCharacter OtherActor))
      (Variables|Default|SetPlayerRef _asbp_third_person_character)))
  (Rendering|SetVisibility (Variables|Default|GetHasKeyB_Message) false false)
  (Rendering|SetVisibility (Variables|Default|GetMissingKeyB_Message) false false)
  (Variables|Default|SetbCanInteract_B false))

(event EventBeginPlay
  ;[0.15 0.15 0.15 0.5] Default Values
  ;;[0.15 0.15 0.15 0.5] UI
  (Rendering|SetVisibility (Variables|Default|GetHasKeyA_Message) false false)
  (Rendering|SetVisibility (Variables|Default|GetMissingKeyA_Message) false false)
  (Rendering|SetVisibility (Variables|Default|GetHasKeyB_Message) false false)
  (Rendering|SetVisibility (Variables|Default|GetMissingKeyB_Message) false false)
  ;;[0.15 0.15 0.15 0.5] Locked Status
  (Variables|Default|SetbUnlockedA false)
  (Variables|Default|SetbUnlockedB false)
  ;;[0.15 0.15 0.15 0.5] Keys
  (Rendering|SetVisibility (Variables|Default|GetKeyA) false false)
  (Rendering|SetVisibility (Variables|Default|GetKeyB) false false))

(event Collision|EventActorBeginOverlap
  (params (OtherActor :type Actor%20Object%20Reference)))

(event EventTick
  (params (DeltaSeconds :type Float%20%28single-precision%29))
  ;[0.15 0.15 0.15 0.5] Check For Player
  (Utilities|IsValid (Variables|Default|GetPlayerRef)
    (:Is%20Valid
      _)
    (:Is%20Not%20Valid
      (bind _asbp_third_person_character (Utilities|Casting|CastToBP_ThirdPersonCharacter (Variables|Default|GetPlayerRef)))
      (bind _output_get (Variables|Default|SetPlayerRef _asbp_third_person_character))))
  ;[0.15 0.15 0.15 0.5] Unlock A
  (if (and (Variables|/Game/ThirdPerson/Blueprints/BP_ThirdPersonCharacter.BP_ThirdPersonCharacter_C|GetbInteraction _output_get) (Variables|Default|GetbCanInteract_A))
    (CallFunction|UseKeyA)
    ;[0.15 0.15 0.15 0.5] Slot Key A Into Place
    (Components|MoveComponentTo (Variables|Default|GetKeyA) "-40.000000,-22.500000,-25.000000" "0, 0, 0" false false 1.0 false))
  ;[0.15 0.15 0.15 0.5] Unlock B
  (if (and (Variables|/Game/ThirdPerson/Blueprints/BP_ThirdPersonCharacter.BP_ThirdPersonCharacter_C|GetbInteraction (Variables|Default|GetPlayerRef)) (Variables|Default|GetbCanInteract_B))
    (CallFunction|UseKeyB)
    ;[0.15 0.15 0.15 0.5] Slot Key B Into Place
    (Components|MoveComponentTo (Variables|Default|GetKeyB) "-40.000000,20.000000,-25.000000" "90.000000,0.000000,0.000000" false false 1.0 false))
  ;[0.15 0.15 0.15 0.5] Open Gate
  (if (and (Variables|Default|GetbUnlockedA) (Variables|Default|GetbUnlockedB))
    (Utilities|FlowControl|Delay 1.0)
    (bind _doorprogress (Timeline|OpenDoorTimeline Play)
      (:Update
        (Transformation|SetRelativeLocation (Variables|Default|GetDoor_R) (Math|Vector|MakeVector 0.0 (Math|Float|Lerp 2e+02 6e+02 _doorprogress) 1.9e+02) false false)
        (Transformation|SetRelativeLocation (Variables|Default|GetDoor_L) (Math|Vector|MakeVector 0.0 (Math|Float|Lerp -2e+02 -6e+02 _doorprogress) 1.9e+02) false false)))))

(fn ConstructionScript)

(fn UseKeyA
  ;[0.15 0.15 0.15 0.5] Check For Player
  (Utilities|IsValid (Variables|Default|GetPlayerRef)
    (:Is%20Valid
      _)
    (:Is%20Not%20Valid
      (bind _asbp_third_person_character (Utilities|Casting|CastToBP_ThirdPersonCharacter (Variables|Default|GetPlayerRef)))
      ;[0.15 0.15 0.15 0.5] Place Key
      (bind _output_get (Variables|Default|SetPlayerRef _asbp_third_person_character))))
  (Rendering|SetVisibility (Variables|Default|GetKeyA) true false)
  ;[0.15 0.15 0.15 0.5] Disable UI
  (Rendering|SetVisibility (Variables|Default|GetHasKeyA_Message) false false)
  ;[0.15 0.15 0.15 0.5] Remove From Inventory
  (Variables|/Game/ThirdPerson/Blueprints/BP_Inventory.BP_Inventory_C|SetKeyA (Variables|/Game/ThirdPerson/Blueprints/BP_ThirdPersonCharacter.BP_ThirdPersonCharacter_C|GetPlayerInventory _output_get) (- (Variables|/Game/ThirdPerson/Blueprints/BP_Inventory.BP_Inventory_C|GetKeyA (Variables|/Game/ThirdPerson/Blueprints/BP_ThirdPersonCharacter.BP_ThirdPersonCharacter_C|GetPlayerInventory _output_get)) 1))
  (Variables|Default|SetbUnlockedA true)
  (return))

(fn UseKeyB
  ;[0.15 0.15 0.15 0.5] Check For Player
  (Utilities|IsValid (Variables|Default|GetPlayerRef)
    (:Is%20Valid
      _)
    (:Is%20Not%20Valid
      (bind _asbp_third_person_character (Utilities|Casting|CastToBP_ThirdPersonCharacter (Variables|Default|GetPlayerRef)))
      ;[0.15 0.15 0.15 0.5] Place Key
      (bind _output_get (Variables|Default|SetPlayerRef _asbp_third_person_character))))
  (Rendering|SetVisibility (Variables|Default|GetKeyB) true false)
  ;[0.15 0.15 0.15 0.5] Disable UI
  (Rendering|SetVisibility (Variables|Default|GetHasKeyB_Message) false false)
  ;[0.15 0.15 0.15 0.5] Remove From Inventory
  (Variables|/Game/ThirdPerson/Blueprints/BP_Inventory.BP_Inventory_C|SetKeyB (Variables|/Game/ThirdPerson/Blueprints/BP_ThirdPersonCharacter.BP_ThirdPersonCharacter_C|GetPlayerInventory _output_get) (- (Variables|/Game/ThirdPerson/Blueprints/BP_Inventory.BP_Inventory_C|GetKeyB (Variables|/Game/ThirdPerson/Blueprints/BP_ThirdPersonCharacter.BP_ThirdPersonCharacter_C|GetPlayerInventory _output_get)) 1))
  (Variables|Default|SetbUnlockedB true)
  (return))