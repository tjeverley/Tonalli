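; Eight-button glyph panel puzzle that the player solves by entering a sequence of glyphs.
; Tick polls Value to either depress that glyph with its light and output, or reset the panel through a timeline on zero.
; CheckSolution, not called within this graph, compares input against the Solution array to mark Complete or restart.
; InteractionDetector overlap toggles the reticule, prompt and player's Panel flag, zeroing Value on exit if unsolved.
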(event OnComponentBeginOverlap(InteractionDetector)
  (params (OverlappedComponent :type Primitive%20Component%20Object%20Reference) (OtherActor :type Actor%20Object%20Reference) (OtherComp :type Primitive%20Component%20Object%20Reference) (OtherBodyIndex :type Integer) (bFromSweep :type Boolean) (SweepResult :type Hit%20Result%20Structure%20%28by%20ref%29))
  ;[0.15 0.15 0.15 0.5] Display/Hide Selection Cursor
  (Utilities|IsValid (Variables|Default|GetPlayerRef)
    (:Is%20Valid
      _)
    (:Is%20Not%20Valid
      (bind _asbp_third_person_character (Utilities|Casting|CastToBP_ThirdPersonCharacter OtherActor))
      (Variables|Default|SetPlayerRef _asbp_third_person_character)))
  (Utilities|IsValid (Variables|Default|GetCrosshairRef)
    (:Is%20Valid
      _)
    (:Is%20Not%20Valid
      (bind _returnvalue (UserInterface|CreateWidget "/Game/UI/WBP_Reticule.WBP_Reticule_C" (Game|GetPlayerController 0)))
      (bind _output_get (Variables|Default|SetCrosshairRef _returnvalue))))
  (UserInterface|Viewport|AddtoViewport _output_get 0)
  (Variables|/Game/ThirdPerson/Blueprints/BP_ThirdPersonCharacter.BP_ThirdPersonCharacter_C|SetbPanel (Variables|Default|GetPlayerRef) true)
  (Rendering|SetVisibility (Variables|Default|GetInteractionMessage) true false))

(event OnComponentEndOverlap(InteractionDetector)
  (params (OverlappedComponent :type Primitive%20Component%20Object%20Reference) (OtherActor :type Actor%20Object%20Reference) (OtherComp :type Primitive%20Component%20Object%20Reference) (OtherBodyIndex :type Integer))
  ;[0.15 0.15 0.15 0.5] Display/Hide Selection Cursor
  (Utilities|IsValid (Variables|Default|GetPlayerRef)
    (:Is%20Valid
      _)
    (:Is%20Not%20Valid
      (bind _asbp_third_person_character (Utilities|Casting|CastToBP_ThirdPersonCharacter OtherActor))
      (Variables|Default|SetPlayerRef _asbp_third_person_character)))
  (Utilities|IsValid (Variables|Default|GetCrosshairRef)
    (:Is%20Valid
      _)
    (:Is%20Not%20Valid
      (bind _returnvalue (UserInterface|CreateWidget "/Game/UI/WBP_Reticule.WBP_Reticule_C" (Game|GetPlayerController 0)))
      (bind _output_get (Variables|Default|SetCrosshairRef _returnvalue))))
  (Widget|RemovefromParent _output_get)
  (Variables|/Game/ThirdPerson/Blueprints/BP_ThirdPersonCharacter.BP_ThirdPersonCharacter_C|SetbPanel (Variables|Default|GetPlayerRef) false)
  (Rendering|SetVisibility (Variables|Default|GetInteractionMessage) false false)
  ;[0.15 0.15 0.15 0.5] Reset Puzzle if Not solved
  (if (not (Variables|Default|GetbComplete))
    (Variables|Default|SetValue 0)))

(event EventBeginPlay
  ;[0.15 0.15 0.15 0.5] Default
  (CallFunction|LightsOff)
  (Rendering|SetVisibility (Variables|Default|GetInteractionMessage) false false))

(event EventTick
  (params (DeltaSeconds :type Float%20%28single-precision%29))
  ;[0.15 0.15 0.15 0.5] Hide UI Once Solved
  (if (Variables|Default|GetbComplete)
    (Rendering|SetVisibility (Variables|Default|GetInteractionMessage) false false))
  ;[0.15 0.15 0.15 0.5] Take Input
  (switch int (Variables|Default|GetValue)
    (:0
      ;[0.15 0.15 0.15 0.5] Reset Panel
      (CallFunction|LightsOff)
      (bind _keysup (Timeline|ResetTimeline Play)
        (:Update
          ;;[0.15 0.15 0.15 0.5] Reset Glyph 1
          (Transformation|SetRelativeLocation (Variables|Default|GetGlyph1) (Math|Vector|MakeVector (Math|Float|Lerp -26.450218 -27.942728 _keysup) -194.05944 (Math|Float|Lerp 45.813122 49.91376 _keysup)) false false)
          ;;[0.15 0.15 0.15 0.5] Reset Glyph 2
          (Transformation|SetRelativeLocation (Variables|Default|GetGlyph2) (Math|Vector|MakeVector (Math|Float|Lerp -26.450218 -27.942728 _keysup) -140.442933 (Math|Float|Lerp 45.813122 49.91376 _keysup)) false false)
          ;;[0.15 0.15 0.15 0.5] Reset Glyph 3
          (Transformation|SetRelativeLocation (Variables|Default|GetGlyph3) (Math|Vector|MakeVector (Math|Float|Lerp -26.450218 -27.942728 _keysup) -85.402442 (Math|Float|Lerp 45.813122 49.91376 _keysup)) false false)
          ;;[0.15 0.15 0.15 0.5] Reset Glyph 4
          (Transformation|SetRelativeLocation (Variables|Default|GetGlyph4) (Math|Vector|MakeVector (Math|Float|Lerp -26.450218 -27.942728 _keysup) -30.762835 (Math|Float|Lerp 45.813122 49.91376 _keysup)) false false)
          ;;[0.15 0.15 0.15 0.5] Reset Glyph 5
          (Transformation|SetRelativeLocation (Variables|Default|GetGlyph5) (Math|Vector|MakeVector (Math|Float|Lerp -26.450218 -27.942728 _keysup) 36.808412 (Math|Float|Lerp 45.813122 49.91376 _keysup)) false false)
          ;;[0.15 0.15 0.15 0.5] Reset Glyph 6
          (Transformation|SetRelativeLocation (Variables|Default|GetGlyph6) (Math|Vector|MakeVector (Math|Float|Lerp -26.450218 -27.942728 _keysup) 90.424919 (Math|Float|Lerp 45.813122 49.91376 _keysup)) false false)
          ;;[0.15 0.15 0.15 0.5] Reset Glyph 7
          (Transformation|SetRelativeLocation (Variables|Default|GetGlyph7) (Math|Vector|MakeVector (Math|Float|Lerp -26.450218 -27.942728 _keysup) 145.46541 (Math|Float|Lerp 45.813122 49.91376 _keysup)) false false)
          ;;[0.15 0.15 0.15 0.5] Reset Glyph 8
          (Transformation|SetRelativeLocation (Variables|Default|GetGlyph8) (Math|Vector|MakeVector (Math|Float|Lerp -26.450218 -27.942728 _keysup) 200.105017 (Math|Float|Lerp 45.813122 49.91376 _keysup)) false false)
          (CallFunction|ResetOutput))))
    (:1
      (Utilities|Depress1))
    (:2
      (Utilities|Depress2))
    (:3
      (Utilities|Depress3))
    (:4
      (Utilities|Depress4))
    (:5
      (Utilities|Depress5))
    (:6
      (Utilities|Depress6))
    (:7
      (Utilities|Depress7))
    (:8
      (Utilities|Depress8))))

(fn ConstructionScript)

(fn CheckSolution
  (params (Value :type Integer))
  ;[0.15 0.15 0.15 0.5] Check Value Against Solution
  (if (== Value (Utilities|Array|Get(acopy) (Variables|Default|GetSolution) (Variables|Default|GetSolutionIndex)))
    (if (== (Variables|Default|GetSolutionIndex) (- (Utilities|Array|Length (Variables|Default|GetSolution)) 1))
      ;[0.15 0.15 0.15 0.5] Mark Puzzle as Solved
      (Variables|Default|SetbComplete true)
      (else
        ;[0.15 0.15 0.15 0.5] Increment Index
        (Variables|Default|SetSolutionIndex (+ (Variables|Default|GetSolutionIndex) 1))))
    (else
      ;[0.15 0.15 0.15 0.5] Reset Puzzle
      (Variables|Default|SetValue 0)
      (Variables|Default|SetSolutionIndex 0)))
  (return))

(fn LightsOff
  (Rendering|Components|Light|SetIntensity (Variables|Default|GetConfirmLight1) 0.0)
  (Rendering|Components|Light|SetIntensity (Variables|Default|GetConfirmLight2) 0.0)
  (Rendering|Components|Light|SetIntensity (Variables|Default|GetConfirmLight3) 0.0)
  (Rendering|Components|Light|SetIntensity (Variables|Default|GetConfirmLight4) 0.0)
  (Rendering|Components|Light|SetIntensity (Variables|Default|GetConfirmLight5) 0.0)
  (Rendering|Components|Light|SetIntensity (Variables|Default|GetConfirmLight6) 0.0)
  (Rendering|Components|Light|SetIntensity (Variables|Default|GetConfirmLight7) 0.0)
  (Rendering|Components|Light|SetIntensity (Variables|Default|GetConfirmLight8) 0.0)
  (return))

(fn ResetOutput
  (Rendering|SetVisibility (Variables|Default|GetOutput1) false false)
  (Rendering|SetVisibility (Variables|Default|GetOutput2) false false)
  (Rendering|SetVisibility (Variables|Default|GetOutput3) false false)
  (Rendering|SetVisibility (Variables|Default|GetOutput4) false false)
  (Rendering|SetVisibility (Variables|Default|GetOutput5) false false)
  (Rendering|SetVisibility (Variables|Default|GetOutput6) false false)
  (Rendering|SetVisibility (Variables|Default|GetOutput7) false false)
  (Rendering|SetVisibility (Variables|Default|GetOutput8) false false)
  (return))