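; Puzzle gate with three key slots (A, B, C) that opens once all three keys from the player's inventory are placed.
; Slot overlaps show has-key or missing-key prompts and set interaction flags based on inventory counts.
; Tick polls the player's Interaction flag to call UseKey functions, which reveal and deduct keys, then slides them into place.
; With all locks set, Tick plays a delayed timeline that lerps both doors apart.
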(event OnComponentBeginOverlap(KeyASlot)
  (params (OverlappedComponent :type Primitive%20Component%20Object%20Reference) (OtherActor :type Actor%20Object%20Reference) (OtherComp :type Primitive%20Component%20Object%20Reference) (OtherBodyIndex :type Integer) (bFromSweep :type Boolean) (SweepResult :type Hit%20Result%20Structure%20%28by%20ref%29))
  (bind _keya (Variables|Default|GetKeyA))
  (bind _returnvalue (Rendering|IsVisible _keya))
  (bind _returnvalue_2 (not _returnvalue))
  ;[0.15 0.15 0.15 0.5] Slot A UI
  ;;[0.15 0.15 0.15 0.5] Display Key Slot A UI
  (Utilities|IsValid (Variables|Default|GetPlayerRef)
    (:Is%20Valid
      _)
    (:Is%20Not%20Valid
      (bind _asbp_third_person_character (Utilities|Casting|CastToBP_ThirdPersonCharacter (Game|GetPlayerCharacter 0)))
      (bind _output_get (Variables|Default|SetPlayerRef _asbp_third_person_character))))
  ;;;[0.15 0.15 0.15 0.5] Check For Keys
  (if (== OtherActor (Variables|Default|GetPlayerRef))
    (if (> (Variables|/Game/ThirdPerson/Blueprints/BP_Inventory.BP_Inventory_C|GetKeyA (Variables|/Game/ThirdPerson/Blueprints/BP_ThirdPersonCharacter.BP_ThirdPersonCharacter_C|GetPlayerInventory _output_get)) 0)
      (Rendering|SetVisibility (Variables|Default|GetHasKeyA_Message) _returnvalue_2 false)
      (Variables|Default|SetbCanInteract_A _returnvalue_2)
      (else
        (Rendering|SetVisibility (Variables|Default|GetMissingKeyA_Message) _returnvalue_2 false)))))

(event OnComponentEndOverlap(KeyASlot)
  (params (OverlappedComponent :type Primitive%20Component%20Object%20Reference) (OtherActor :type Actor%20Object%20Reference) (OtherComp :type Primitive%20Component%20Object%20Reference) (OtherBodyIndex :type Integer))
  ;[0.15 0.15 0.15 0.5] Slot A UI
  ;;[0.15 0.15 0.15 0.5] Hide Key Slot A UI
  (Utilities|IsValid (Variables|Default|GetPlayerRef)
    (:Is%20Valid
      _)
    (:Is%20Not%20Valid
      (bind _asbp_third_person_character (Utilities|Casting|CastToBP_ThirdPersonCharacter (Game|GetPlayerCharacter 0)))
      (Variables|Default|SetPlayerRef _asbp_third_person_character)))
  (if (== OtherActor (Variables|Default|GetPlayerRef))
    (Rendering|SetVisibility (Variables|Default|GetHasKeyA_Message) false false)
    (Rendering|SetVisibility (Variables|Default|GetMissingKeyA_Message) false false)
    (Variables|Default|SetbCanInteract_A false)))

(event OnComponentBeginOverlap(KeyBSlot)
  (params (OverlappedComponent :type Primitive%20Component%20Object%20Reference) (OtherActor :type Actor%20Object%20Reference) (OtherComp :type Primitive%20Component%20Object%20Reference) (OtherBodyIndex :type Integer) (bFromSweep :type Boolean) (SweepResult :type Hit%20Result%20Structure%20%28by%20ref%29))
  (bind _keyb (Variables|Default|GetKeyB))
  (bind _returnvalue (Rendering|IsVisible _keyb))
  (bind _returnvalue_2 (not _returnvalue))
  ;[0.15 0.15 0.15 0.5] Slot B UI
  ;;[0.15 0.15 0.15 0.5] Display Key Slot B UI
  (Utilities|IsValid (Variables|Default|GetPlayerRef)
    (:Is%20Valid
      _)
    (:Is%20Not%20Valid
      (bind _asbp_third_person_character (Utilities|Casting|CastToBP_ThirdPersonCharacter (Game|GetPlayerCharacter 0)))
      (bind _output_get (Variables|Default|SetPlayerRef _asbp_third_person_character))))
  ;;;[0.15 0.15 0.15 0.5] Check For Keys
  (if (== OtherActor (Variables|Default|GetPlayerRef))
    (if (> (Variables|/Game/ThirdPerson/Blueprints/BP_Inventory.BP_Inventory_C|GetKeyB (Variables|/Game/ThirdPerson/Blueprints/BP_ThirdPersonCharacter.BP_ThirdPersonCharacter_C|GetPlayerInventory _output_get)) 0)
      (Rendering|SetVisibility (Variables|Default|GetHasKeyB_Message) _returnvalue_2 false)
      (Variables|Default|SetbCanInteract_B _returnvalue_2)
      (else
        (Rendering|SetVisibility (Variables|Default|GetMissingKeyB_Message) _returnvalue_2 false)))))

(event OnComponentEndOverlap(KeyBSlot)
  (params (OverlappedComponent :type Primitive%20Component%20Object%20Reference) (OtherActor :type Actor%20Object%20Reference) (OtherComp :type Primitive%20Component%20Object%20Reference) (OtherBodyIndex :type Integer))
  ;[0.15 0.15 0.15 0.5] Slot B UI
  ;;[0.15 0.15 0.15 0.5] Hide Key Slot B UI
  (Utilities|IsValid (Variables|Default|GetPlayerRef)
    (:Is%20Valid
      _)
    (:Is%20Not%20Valid
      (bind _asbp_third_person_character (Utilities|Casting|CastToBP_ThirdPersonCharacter (Game|GetPlayerCharacter 0)))
      (Variables|Default|SetPlayerRef _asbp_third_person_character)))
  (if (== OtherActor (Variables|Default|GetPlayerRef))
    (Rendering|SetVisibility (Variables|Default|GetHasKeyB_Message) false false)
    (Rendering|SetVisibility (Variables|Default|GetMissingKeyB_Message) false false)
    (Variables|Default|SetbCanInteract_B false)))

(event OnComponentBeginOverlap(KeyCSlot)
  (params (OverlappedComponent :type Primitive%20Component%20Object%20Reference) (OtherActor :type Actor%20Object%20Reference) (OtherComp :type Primitive%20Component%20Object%20Reference) (OtherBodyIndex :type Integer) (bFromSweep :type Boolean) (SweepResult :type Hit%20Result%20Structure%20%28by%20ref%29))
  (bind _keyc (Variables|Default|GetKeyC))
  (bind _returnvalue (Rendering|IsVisible _keyc))
  (bind _returnvalue_2 (not _returnvalue))
  ;[0.15 0.15 0.15 0.5] Slot C UI
  ;;[0.15 0.15 0.15 0.5] Display Key Slot C UI
  (Utilities|IsValid (Variables|Default|GetPlayerRef)
    (:Is%20Valid
      _)
    (:Is%20Not%20Valid
      (bind _asbp_third_person_character (Utilities|Casting|CastToBP_ThirdPersonCharacter (Game|GetPlayerCharacter 0)))
      (bind _output_get (Variables|Default|SetPlayerRef _asbp_third_person_character))))
  ;;;[0.15 0.15 0.15 0.5] Check For Keys
  (if (== OtherActor (Variables|Default|GetPlayerRef))
    (if (> (Variables|/Game/ThirdPerson/Blueprints/BP_Inventory.BP_Inventory_C|GetKeyC (Variables|/Game/ThirdPerson/Blueprints/BP_ThirdPersonCharacter.BP_ThirdPersonCharacter_C|GetPlayerInventory _output_get)) 0)
      (Rendering|SetVisibility (Variables|Default|GetHasKeyC_Message) _returnvalue_2 false)
      (Variables|Default|SetbCanInteract_C _returnvalue_2)
      (else
        (Rendering|SetVisibility (Variables|Default|GetMissingKeyC_Message) _returnvalue_2 false)))))

(event OnComponentEndOverlap(KeyCSlot)
  (params (OverlappedComponent :type Primitive%20Component%20Object%20Reference) (OtherActor :type Actor%20Object%20Reference) (OtherComp :type Primitive%20Component%20Object%20Reference) (OtherBodyIndex :type Integer))
  ;[0.15 0.15 0.15 0.5] Slot C UI
  ;;[0.15 0.15 0.15 0.5] Hide Key Slot C UI
  (Utilities|IsValid (Variables|Default|GetPlayerRef)
    (:Is%20Valid
      _)
    (:Is%20Not%20Valid
      (bind _asbp_third_person_character (Utilities|Casting|CastToBP_ThirdPersonCharacter (Game|GetPlayerCharacter 0)))
      (Variables|Default|SetPlayerRef _asbp_third_person_character)))
  (if (== OtherActor (Variables|Default|GetPlayerRef))
    (Rendering|SetVisibility (Variables|Default|GetHasKeyC_Message) false false)
    (Rendering|SetVisibility (Variables|Default|GetMissingKeyC_Message) false false)
    (Variables|Default|SetbCanInteract_C false)))

(event EventBeginPlay
  ;[0.15 0.15 0.15 0.5] Default Values
  ;;[0.15 0.15 0.15 0.5] UI
  (Rendering|SetVisibility (Variables|Default|GetHasKeyA_Message) false false)
  (Rendering|SetVisibility (Variables|Default|GetMissingKeyA_Message) false false)
  (Rendering|SetVisibility (Variables|Default|GetHasKeyB_Message) false false)
  (Rendering|SetVisibility (Variables|Default|GetMissingKeyB_Message) false false)
  (Rendering|SetVisibility (Variables|Default|GetHasKeyC_Message) false false)
  (Rendering|SetVisibility (Variables|Default|GetMissingKeyC_Message) false false)
  ;;[0.15 0.15 0.15 0.5] Locked Status
  (Variables|Default|SetbUnlockedA false)
  (Variables|Default|SetbUnlockedB false)
  (Variables|Default|SetbUnlocked_C false)
  ;;[0.15 0.15 0.15 0.5] Keys
  (Rendering|SetVisibility (Variables|Default|GetKeyA) false false)
  (Rendering|SetVisibility (Variables|Default|GetKeyB) false false)
  (Rendering|SetVisibility (Variables|Default|GetKeyC) false false))

(event Collision|EventActorBeginOverlap
  (params (OtherActor :type Actor%20Object%20Reference)))

(event EventTick
  (params (DeltaSeconds :type Float%20%28single-precision%29))
  ;[0.15 0.15 0.15 0.5] Check For Player
  (Utilities|IsValid (Variables|Default|GetPlayerRef)
    (:Is%20Valid
      _)
    (:Is%20Not%20Valid
      (bind _asbp_third_person_character (Utilities|Casting|CastToBP_ThirdPersonCharacter (Game|GetPlayerCharacter 0)))
      (bind _output_get (Variables|Default|SetPlayerRef _asbp_third_person_character))))
  ;[0.15 0.15 0.15 0.5] Unlock A
  (if (and (Variables|/Game/ThirdPerson/Blueprints/BP_ThirdPersonCharacter.BP_ThirdPersonCharacter_C|GetbInteraction _output_get) (Variables|Default|GetbCanInteract_A))
    (CallFunction|UseKeyA)
    ;[0.15 0.15 0.15 0.5] Slot Key A Into Place
    (Components|MoveComponentTo (Variables|Default|GetKeyA) "244.841793,-39.351751,92.565399" "0, 0, 0" false false 1.0 false))
  ;[0.15 0.15 0.15 0.5] Unlock B
  (if (and (Variables|/Game/ThirdPerson/Blueprints/BP_ThirdPersonCharacter.BP_ThirdPersonCharacter_C|GetbInteraction (Variables|Default|GetPlayerRef)) (Variables|Default|GetbCanInteract_B))
    (CallFunction|UseKeyB)
    ;[0.15 0.15 0.15 0.5] Slot Key B Into Place
    (Components|MoveComponentTo (Variables|Default|GetKeyB) "253.625687,-38.829736,91.158026" "0, 0, 0" false false 1.0 false))
  ;[0.15 0.15 0.15 0.5] Unlock C
  (if (and (Variables|/Game/ThirdPerson/Blueprints/BP_ThirdPersonCharacter.BP_ThirdPersonCharacter_C|GetbInteraction (Variables|Default|GetPlayerRef)) (Variables|Default|GetbCanInteract_C))
    (CallFunction|UseKeyC)
    ;[0.15 0.15 0.15 0.5] Slot Key C Into Place
    (Components|MoveComponentTo (Variables|Default|GetKeyC) "542.277691,-38.368186,92.565399" "0, 0, 0" false false 1.0 false))
  ;[0.15 0.15 0.15 0.5] Open Gate
  (if (Math|Boolean|ANDBoolean (Variables|Default|GetbUnlockedA) (Variables|Default|GetbUnlockedB) (Variables|Default|GetbUnlocked_C))
    (Utilities|FlowControl|Delay 1.0)
    (bind _doorprogress (Timeline|OpenDoorTimeline Play)
      (:Update
        (Transformation|SetRelativeLocation (Variables|Default|GetDoor_R) (Math|Vector|MakeVector -57.610138 (Math|Float|Lerp 527.285045 862.370899 _doorprogress) 1.120925) false false)
        (Transformation|SetRelativeLocation (Variables|Default|GetDoor_L) (Math|Vector|MakeVector -58.315536 (Math|Float|Lerp -528.720748 -783.376599 _doorprogress) -0.251264) false false)))))

(fn ConstructionScript)

(fn UseKeyA
  ;[0.15 0.15 0.15 0.5] Check For Player
  (Utilities|IsValid (Variables|Default|GetPlayerRef)
    (:Is%20Valid
      _)
    (:Is%20Not%20Valid
      (bind _asbp_third_person_character (Utilities|Casting|CastToBP_ThirdPersonCharacter (Game|GetPlayerCharacter 0)))
      ;[0.15 0.15 0.15 0.5] Place Key
      (bind _output_get (Variables|Default|SetPlayerRef _asbp_third_person_character))))
  (Rendering|SetVisibility (Variables|Default|GetKeyA) true false)
  ;[0.15 0.15 0.15 0.5] Disable UI
  (Rendering|SetVisibility (Variables|Default|GetHasKeyA_Message) false false)
  ;[0.15 0.15 0.15 0.5] Remove From Inventory
  (Variables|/Game/ThirdPerson/Blueprints/BP_Inventory.BP_Inventory_C|SetKeyA (Variables|/Game/ThirdPerson/Blueprints/BP_ThirdPersonCharacter.BP_ThirdPersonCharacter_C|GetPlayerInventory _output_get) (- (Variables|/Game/ThirdPerson/Blueprints/BP_Inventory.BP_Inventory_C|GetKeyA (Variables|/Game/ThirdPerson/Blueprints/BP_ThirdPersonCharacter.BP_ThirdPersonCharacter_C|GetPlayerInventory _output_get)) 1))
  (Variables|Default|SetbUnlockedA true)
  (return))

(fn UseKeyB
  ;[0.15 0.15 0.15 0.5] Check For Player
  (Utilities|IsValid (Variables|Default|GetPlayerRef)
    (:Is%20Valid
      _)
    (:Is%20Not%20Valid
      (bind _asbp_third_person_character (Utilities|Casting|CastToBP_ThirdPersonCharacter (Game|GetPlayerCharacter 0)))
      ;[0.15 0.15 0.15 0.5] Place Key
      (bind _output_get (Variables|Default|SetPlayerRef _asbp_third_person_character))))
  (Rendering|SetVisibility (Variables|Default|GetKeyB) true false)
  ;[0.15 0.15 0.15 0.5] Disable UI
  (Rendering|SetVisibility (Variables|Default|GetHasKeyB_Message) false false)
  ;[0.15 0.15 0.15 0.5] Remove From Inventory
  (Variables|/Game/ThirdPerson/Blueprints/BP_Inventory.BP_Inventory_C|SetKeyB (Variables|/Game/ThirdPerson/Blueprints/BP_ThirdPersonCharacter.BP_ThirdPersonCharacter_C|GetPlayerInventory _output_get) (- (Variables|/Game/ThirdPerson/Blueprints/BP_Inventory.BP_Inventory_C|GetKeyB (Variables|/Game/ThirdPerson/Blueprints/BP_ThirdPersonCharacter.BP_ThirdPersonCharacter_C|GetPlayerInventory _output_get)) 1))
  (Variables|Default|SetbUnlockedB true)
  (return))

(fn UseKeyC
  ;[0.15 0.15 0.15 0.5] Check For Player
  (Utilities|IsValid (Variables|Default|GetPlayerRef)
    (:Is%20Valid
      _)
    (:Is%20Not%20Valid
      (bind _asbp_third_person_character (Utilities|Casting|CastToBP_ThirdPersonCharacter (Game|GetPlayerCharacter 0)))
      ;[0.15 0.15 0.15 0.5] Place Key
      (bind _output_get (Variables|Default|SetPlayerRef _asbp_third_person_character))))
  (Rendering|SetVisibility (Variables|Default|GetKeyC) true false)
  ;[0.15 0.15 0.15 0.5] Disable UI
  (Rendering|SetVisibility (Variables|Default|GetHasKeyC_Message) false false)
  ;[0.15 0.15 0.15 0.5] Remove From Inventory
  (Variables|/Game/ThirdPerson/Blueprints/BP_Inventory.BP_Inventory_C|SetKeyC (Variables|/Game/ThirdPerson/Blueprints/BP_ThirdPersonCharacter.BP_ThirdPersonCharacter_C|GetPlayerInventory _output_get) (- (Variables|/Game/ThirdPerson/Blueprints/BP_Inventory.BP_Inventory_C|GetKeyC (Variables|/Game/ThirdPerson/Blueprints/BP_ThirdPersonCharacter.BP_ThirdPersonCharacter_C|GetPlayerInventory _output_get)) 1))
  (Variables|Default|SetbUnlocked_C true))