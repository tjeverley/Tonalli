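; Puzzle ratchet capstan whose rotation moves a linked object, such as a lifted item, along a chosen X, Y or Z axis.
; Each Tick maps the spine's absolute yaw, scaled by a pulley multiplier, to a clamped offset from the object's starting position.
; Optional cog wall or glyph panel dependencies lock the capstan by toggling spine physics until that puzzle is complete.
; An optional trigger shows the player a one-time tutorial dialogue.
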(event OnComponentBeginOverlap(TutorialTrigger)
  (params (OverlappedComponent :type Primitive%20Component%20Object%20Reference) (OtherActor :type Actor%20Object%20Reference) (OtherComp :type Primitive%20Component%20Object%20Reference) (OtherBodyIndex :type Integer) (bFromSweep :type Boolean) (SweepResult :type Hit%20Result%20Structure%20%28by%20ref%29))
  ;[0.15 0.15 0.15 0.5] Tutorial
  (if (Variables|Default|GetbShowTutorial)
    (CallFunction|Tutorial OtherActor)))

(event EventBeginPlay
  (bind _movedobject (Variables|Default|GetMovedObject))
  (bind _returnvalue (Transformation|GetActorLocation _movedobject))
  (Variables|/Game/Blueprints/Tutorials/BP_Tutorial.BP_Tutorial_C|SetbDismissed (Variables|Default|GetBP_Tutorial) (not (Variables|Default|GetbShowTutorial)))
  ;[0.15 0.15 0.15 0.5] Default Rotation
  (if (Variables|Default|GetbInvert)
    (Transformation|SetRelativeRotation (Variables|Default|GetSpine) "0.000000,180.000000,0.000000" false false))
  ;[0.15 0.15 0.15 0.5] Get Lifted Item Starting Position
  (switch Utilities|FlowControl|Switch|SwitchonBP_EnumAxes (Variables|Default|GetDirection)
    (:NewEnumerator0
      (Variables|Default|SetBaseX (.x _returnvalue)))
    (:NewEnumerator1
      (Variables|Default|SetBaseY (.y _returnvalue)))
    (:NewEnumerator2
      (Variables|Default|SetBaseZ (.z _returnvalue)))))

(event Collision|EventActorBeginOverlap
  (params (OtherActor :type Actor%20Object%20Reference)))

(event EventTick
  (params (DeltaSeconds :type Float%20%28single-precision%29))
  (bind _spine (Variables|Default|GetSpine))
  (bind _relativerotation (Variables|/Script/Engine.SceneComponent|GetRelativeRotation _spine))
  (bind _returnvalue (Math|Float|Absolute(Float) (.yaw _relativerotation)))
  ;[0.15 0.15 0.15 0.5] Get Capstan Rotation Angle
  (CallFunction|Lock)
  (switch Utilities|FlowControl|Switch|SwitchonBP_EnumAxes (Variables|Default|GetDirection)
    (:NewEnumerator0
      (CallFunction|MoveonX _returnvalue))
    (:NewEnumerator1
      (CallFunction|MoveonY _returnvalue))
    (:NewEnumerator2
      (CallFunction|MoveonZ _returnvalue))))

(fn ConstructionScript)

(fn MoveonZ
  (params (RotationAngle :type Float%20%28double-precision%29))
  (bind _movedobject (Variables|Default|GetMovedObject))
  (bind _basez (Variables|Default|GetBaseZ))
  (bind _returnvalue (Transformation|GetActorLocation _movedobject))
  ;[0.15 0.15 0.15 0.5] Set Lifted Item Position
  (Transformation|SetActorLocation _movedobject (Math|Vector|MakeVector (.x _returnvalue) (.y _returnvalue) (Math|Float|Clamp(Float) (- (* (+ _basez RotationAngle) (Variables|Default|GetPulleyMultiplier)) (* (Variables|Default|GetBaseZ) (- (Variables|Default|GetPulleyMultiplier) 1.0))) _basez (* (+ _basez RotationAngle) (Variables|Default|GetPulleyMultiplier)))) false false)
  (return))

(fn MoveonY
  (params (RotationAngle :type Float%20%28double-precision%29))
  (bind _basey (Variables|Default|GetBaseY))
  (bind _movedobject (Variables|Default|GetMovedObject))
  (bind _returnvalue (Transformation|GetActorLocation _movedobject))
  ;[0.15 0.15 0.15 0.5] Set Lifted Item Position
  (Transformation|SetActorLocation _movedobject (Math|Vector|MakeVector (.x _returnvalue) (Math|Float|Clamp(Float) (- (* (+ _basey RotationAngle) (Variables|Default|GetPulleyMultiplier)) (* (Variables|Default|GetBaseY) (- (Variables|Default|GetPulleyMultiplier) 1.0))) _basey (* (+ _basey RotationAngle) (Variables|Default|GetPulleyMultiplier))) (.z _returnvalue)) false false)
  (return))

(fn MoveonX
  (params (RotationAngle :type Float%20%28double-precision%29))
  (bind _basex (Variables|Default|GetBaseX))
  (bind _movedobject (Variables|Default|GetMovedObject))
  (bind _returnvalue (Transformation|GetActorLocation _movedobject))
  ;[0.15 0.15 0.15 0.5] Set Lifted Item Position
  (Transformation|SetActorLocation _movedobject (Math|Vector|MakeVector (Math|Float|Clamp(Float) (- (* (+ _basex RotationAngle) (Variables|Default|GetPulleyMultiplier)) (* (Variables|Default|GetBaseX) (- (Variables|Default|GetPulleyMultiplier) 1.0))) _basex (* (+ _basex RotationAngle) (Variables|Default|GetPulleyMultiplier))) (.y _returnvalue) (.z _returnvalue)) false false)
  (return))

(fn Lock
  (bind _glyphpanelref (Variables|Default|GetGlyphPanelRef))
  (bind _spine (Variables|Default|GetSpine))
  (bind _cogwallref (Variables|Default|GetCogWallRef))
  (if (Variables|Default|GetbCogDependent)
    (Utilities|IsValid _cogwallref
      (:Is%20Valid
        (if (Variables|/Game/Blueprints/Puzzles/BP_CogWall.BP_CogWall_C|GetbComplete _cogwallref)
          (Physics|SetSimulatePhysics _spine true :!label _label)
          (else
            (Physics|SetSimulatePhysics _spine false :!label _label_2)))))
    (elif (Variables|Default|GetbGlyphDependent)
      (Utilities|IsValid _glyphpanelref
        (:Is%20Valid
          (if (Variables|/Game/Blueprints/Puzzles/BP_GlyphPanel.BP_GlyphPanel_C|GetbComplete _glyphpanelref)
            (goto _label)
            (else
              (goto _label_2)))))
      (else
        _)))
  (return))

(fn Tutorial
  (params (Player :type Actor%20Object%20Reference))
  (bind _bp_tutorial (Variables|Default|GetBP_Tutorial))
  ;[0.15 0.15 0.15 0.5] Check for Player
  (Utilities|IsValid (Variables|Default|GetPlayerRef)
    (:Is%20Valid
      _)
    (:Is%20Not%20Valid
      (bind _asbp_third_person_character (Utilities|Casting|CastToBP_ThirdPersonCharacter (Game|GetPlayerCharacter 0)))
      (bind _output_get (Variables|Default|SetPlayerRef _asbp_third_person_character))))
  (if (== Player _output_get)
    (Variables|/Game/ThirdPerson/Blueprints/BP_ThirdPersonCharacter.BP_ThirdPersonCharacter_C|SetbDialogue _output_get true)
    (if (Variables|/Game/Blueprints/Tutorials/BP_Tutorial.BP_Tutorial_C|GetbDismissed _bp_tutorial)
      (return)
      (else
        (Default|ShowTutorial _bp_tutorial)
        (Default|DialogueBox (Variables|Default|GetPlayerRef))
        (Variables|/Game/Blueprints/Tutorials/BP_Tutorial.BP_Tutorial_C|SetbDismissed (Variables|Default|GetBP_Tutorial) true)
        (return)))
    (else
      (return))))