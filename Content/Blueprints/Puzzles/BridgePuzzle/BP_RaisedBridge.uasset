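; Puzzle bridge platform that slides its Cube between a raised and a lowered height according to the Raised flag.
; BeginPlay snaps the Cube to the height matching that flag.
; Tick checks the flag every frame and drives two opposing timed MoveComponentTo nodes, calling Return on one and Move on the other to ease toward the current target.
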(event EventBeginPlay
  (bind _cube (Variables|Default|GetCube))
  ;[0.15 0.15 0.15 0.5] Set Starting Height
  (if (Variables|Default|GetbRaised)
    (Transformation|SetRelativeLocation _cube (Variables|Default|GetRaisedHeight) false false)
    (else
      (Transformation|SetRelativeLocation _cube (Variables|Default|GetLoweredHeight) false false))))

(event EventTick
  (params (DeltaSeconds :type Float%20%28single-precision%29))
  (bind _cube (Variables|Default|GetCube))
  (bind _relativerotation (Variables|/Script/Engine.SceneComponent|GetRelativeRotation _cube))
  ;[0.15 0.15 0.15 0.5] Raise/Lower Platform
  (if (Variables|Default|GetbRaised)
    (Utilities|FlowControl|Sequence
      (:then_0
        (goto _label_2 Return))
      (:then_1
        (Components|MoveComponentTo _cube (Variables|Default|GetRaisedHeight) _relativerotation false false 3.0 false :!label _label)))
    (else
      (Utilities|FlowControl|Sequence
        (:then_0
          (goto _label Return))
        (:then_1
          (Components|MoveComponentTo _cube (Variables|Default|GetLoweredHeight) _relativerotation false false 3.0 false :!label _label_2))))))

(fn ConstructionScript)