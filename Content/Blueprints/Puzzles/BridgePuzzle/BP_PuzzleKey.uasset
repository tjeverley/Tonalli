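; Carryable key piece for the bridge puzzle that the third-person player can pick up and drop.
; An overlap detector shows a camera-facing prompt while the player's hands are empty, and Tick polls the player's Interaction flag to trigger pickup.
; Pickup attaches the actor to the player and records it as CarriedBlock.
; DropBlock, not called here, detaches that block at the player's feet and re-enables its detector.
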(event OnComponentBeginOverlap(InteractionDetector)
  (params (OverlappedComponent :type Primitive%20Component%20Object%20Reference) (OtherActor :type Actor%20Object%20Reference) (OtherComp :type Primitive%20Component%20Object%20Reference) (OtherBodyIndex :type Integer) (bFromSweep :type Boolean) (SweepResult :type Hit%20Result%20Structure%20%28by%20ref%29))
  (bind _playerref (Variables|Default|GetPlayerRef))
  ;[0.15 0.15 0.15 0.5] Display/Hide UI
  (if (== OtherActor _playerref)
    (if (not (Variables|/Game/ThirdPerson/Blueprints/BP_ThirdPersonCharacter.BP_ThirdPersonCharacter_C|GetbCarrying _playerref))
      (CallFunction|WidgetFacePlayer)
      (Rendering|SetVisibility (Variables|Default|GetInteractionMessage) true false)
      (Variables|Default|SetbCanInteract true))))

(event OnComponentEndOverlap(InteractionDetector)
  (params (OverlappedComponent :type Primitive%20Component%20Object%20Reference) (OtherActor :type Actor%20Object%20Reference) (OtherComp :type Primitive%20Component%20Object%20Reference) (OtherBodyIndex :type Integer))
  (bind _playerref (Variables|Default|GetPlayerRef))
  ;[0.15 0.15 0.15 0.5] Display/Hide UI
  (if (== OtherActor _playerref)
    (if (not (Variables|/Game/ThirdPerson/Blueprints/BP_ThirdPersonCharacter.BP_ThirdPersonCharacter_C|GetbCarrying _playerref))
      (Rendering|SetVisibility (Variables|Default|GetInteractionMessage) false false)
      (Variables|Default|SetbCanInteract false))))

(event EventBeginPlay
  ;[0.15 0.15 0.15 0.5] Get Player
  (Utilities|IsValid (Variables|Default|GetPlayerRef)
    (:Is%20Not%20Valid
      (bind _asbp_third_person_character (Utilities|Casting|CastToBP_ThirdPersonCharacter (Game|GetPlayerCharacter 0)))
      (Variables|Default|SetPlayerRef _asbp_third_person_character))))

(event Collision|EventActorBeginOverlap
  (params (OtherActor :type Actor%20Object%20Reference)))

(event EventTick
  (params (DeltaSeconds :type Float%20%28single-precision%29))
  (if (and (Variables|/Game/ThirdPerson/Blueprints/BP_ThirdPersonCharacter.BP_ThirdPersonCharacter_C|GetbInteraction (Variables|Default|GetPlayerRef)) (Variables|Default|GetbCanInteract))
    (CallFunction|PickUpBlock)))

(fn ConstructionScript)

(fn WidgetFacePlayer
  ;[0.15 0.15 0.15 0.5] Orient UI to Face Player
  (Transformation|SetWorldRotation (Variables|Default|GetInteractionMessage) (Math|Rotator|FindLookatRotation (Transformation|GetWorldLocation (Variables|Default|GetInteractionMessage)) (Transformation|GetWorldLocation (Variables|/Script/Engine.PlayerCameraManager|GetTransformComponent (Game|GetPlayerCameraManager 0)))) false false)
  (return))

(fn PickUpBlock
  (bind _playerref (Variables|Default|GetPlayerRef))
  (bind _puzzlepiece (Variables|Default|GetPuzzlePiece))
  (if (Variables|/Game/ThirdPerson/Blueprints/BP_ThirdPersonCharacter.BP_ThirdPersonCharacter_C|GetbCarrying (Variables|Default|GetPlayerRef))
    (return)
    (else
      (if (Class|Actor|IsChildActor self)
        (Transformation|DetachFromActor self "KeepWorld" "KeepWorld" "KeepWorld"))
      (Collision|SetCollisionEnabled (Variables|Default|GetPuzzlePiece) "NoCollision")
      (Transformation|AttachActorToActor (Variables|Default|GetPlayerRef) "None" "SnapToTarget" "SnapToTarget" "KeepWorld" true)
      (Variables|/Game/ThirdPerson/Blueprints/BP_ThirdPersonCharacter.BP_ThirdPersonCharacter_C|SetbCarrying _playerref true)
      (Variables|/Game/ThirdPerson/Blueprints/BP_ThirdPersonCharacter.BP_ThirdPersonCharacter_C|SetCarriedBlock _playerref self)
      (Transformation|SetRelativeRotation _puzzlepiece "90.000000,0.000000,0.000000" false false)
      (Transformation|SetRelativeLocation _puzzlepiece "-30.000000,0.000000,0.000000" false false)
      (Rendering|SetVisibility (Variables|Default|GetInteractionMessage) false false)
      (Collision|SetCollisionEnabled (Variables|Default|GetInteractionDetector) "NoCollision")
      (return))))

(fn DropBlock
  (bind _returnvalue (Game|Player|GetPlayerPawn 0))
  (bind _playerref (Variables|Default|GetPlayerRef))
  (bind _returnvalue_2 (Transformation|GetActorLocation _returnvalue))
  (bind (_origin _boxextent) (Collision|GetActorBounds _returnvalue false false))
  (Transformation|DetachFromActor (Variables|/Game/ThirdPerson/Blueprints/BP_ThirdPersonCharacter.BP_ThirdPersonCharacter_C|GetCarriedBlock (Variables|Default|GetPlayerRef)) "KeepWorld" "KeepWorld" "KeepWorld")
  (Collision|SetCollisionEnabled (Variables|BP_PuzzleKey_C|GetInteractionDetector (Variables|/Game/ThirdPerson/Blueprints/BP_ThirdPersonCharacter.BP_ThirdPersonCharacter_C|GetCarriedBlock (Variables|Default|GetPlayerRef))) "QueryAndPhysics")
  (Transformation|SetActorRelativeLocation (Variables|/Game/ThirdPerson/Blueprints/BP_ThirdPersonCharacter.BP_ThirdPersonCharacter_C|GetCarriedBlock (Variables|Default|GetPlayerRef)) (Math|Vector|MakeVector (.x _returnvalue_2) (.y _returnvalue_2) (+ (- (.z _origin) (.z _boxextent)) 2e+01)))
  (Transformation|SetRelativeRotation (Variables|BP_PuzzleKey_C|GetPuzzlePiece (Variables|/Game/ThirdPerson/Blueprints/BP_ThirdPersonCharacter.BP_ThirdPersonCharacter_C|GetCarriedBlock (Variables|Default|GetPlayerRef))) "180.000000,0.000000,0.000000" false false)
  (Transformation|SetRelativeLocation (Variables|BP_PuzzleKey_C|GetPuzzlePiece (Variables|/Game/ThirdPerson/Blueprints/BP_ThirdPersonCharacter.BP_ThirdPersonCharacter_C|GetCarriedBlock (Variables|Default|GetPlayerRef))) "0, 0, 0" false false)
  (Variables|/Game/ThirdPerson/Blueprints/BP_ThirdPersonCharacter.BP_ThirdPersonCharacter_C|SetbCarrying _playerref false)
  (Variables|/Game/ThirdPerson/Blueprints/BP_ThirdPersonCharacter.BP_ThirdPersonCharacter_C|SetCarriedBlock _playerref 0)
  (return))