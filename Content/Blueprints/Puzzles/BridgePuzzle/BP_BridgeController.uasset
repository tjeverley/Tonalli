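; Puzzle controller panel where BP_PuzzleKey blocks in a 4x4 set of slots decide which bridges are raised.
; On BeginPlay it builds the slot array, spawning attached keys and raising bridges for slots flagged Full.
; Tick polls each slot for an attached child to update Full and each bridge's Raised state.
; PlaceBlock swaps the player's carried block for a new attached key; the trigger toggles the reticule and player panel mode.
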(event OnComponentBeginOverlap(Trigger)
  (params (OverlappedComponent :type Primitive%20Component%20Object%20Reference) (OtherActor :type Actor%20Object%20Reference) (OtherComp :type Primitive%20Component%20Object%20Reference) (OtherBodyIndex :type Integer) (bFromSweep :type Boolean) (SweepResult :type Hit%20Result%20Structure%20%28by%20ref%29))
  (if (== OtherActor (Variables|Default|GetPlayerRef))
    (Variables|Default|SetbCanInteract true)
    (CallFunction|ShowUI)))

(event OnComponentEndOverlap(Trigger)
  (params (OverlappedComponent :type Primitive%20Component%20Object%20Reference) (OtherActor :type Actor%20Object%20Reference) (OtherComp :type Primitive%20Component%20Object%20Reference) (OtherBodyIndex :type Integer))
  (if (== OtherActor (Variables|Default|GetPlayerRef))
    (Variables|Default|SetbCanInteract false)
    (CallFunction|HideUI)))

(event EventBeginPlay
  (Utilities|IsValid (Variables|Default|GetPlayerRef)
    (:Is%20Valid
      _)
    (:Is%20Not%20Valid
      (bind _asbp_third_person_character (Utilities|Casting|CastToBP_ThirdPersonCharacter (Game|GetPlayerCharacter 0)))
      (Variables|Default|SetPlayerRef _asbp_third_person_character)))
  (CallFunction|DefineArrays))

(event Collision|EventActorBeginOverlap
  (params (OtherActor :type Actor%20Object%20Reference)))

(event EventTick
  (params (DeltaSeconds :type Float%20%28single-precision%29))
  (CallFunction|CheckSlots))

(fn ConstructionScript)

(fn DefineArrays
  (bind _bfull (Variables|Default|GetbFull))
  ;[0.15 0.15 0.15 0.5] Populate Slot Array
  (Variables|Default|SetSlots (Utilities|Array|MakeArray (Variables|Default|GetSlot1A) (Variables|Default|GetSlot1B) (Variables|Default|GetSlot1C) (Variables|Default|GetSlot1D) (Variables|Default|GetSlot2A) (Variables|Default|GetSlot2B) (Variables|Default|GetSlot2C) (Variables|Default|GetSlot2D) (Variables|Default|GetSlot3A) (Variables|Default|GetSlot3B) (Variables|Default|GetSlot3C) (Variables|Default|GetSlot3D) (Variables|Default|GetSlot4A) (Variables|Default|GetSlot4B) (Variables|Default|GetSlot4C) (Variables|Default|GetSlot4D)))
  ;[0.15 0.15 0.15 0.5] Check Which Slots Start Filled
  (for _index (range 0 (- (Utilities|Array|Length _bfull) 1))
    (if (Utilities|Array|Get(acopy) _bfull _index)
      ;[0.15 0.15 0.15 0.5] Spawn Blocks in Necessary Slots
      (bind _returnvalue (Game|SpawnActorfromClass "/Game/Blueprints/Puzzles/BridgePuzzle/BP_PuzzleKey.BP_PuzzleKey_C" (Math|Transform|MakeTransform (+ (Transformation|GetWorldLocation (Utilities|Array|Get(acopy) (Variables|Default|GetSlots) _index)) (Math|Vector|MakeVector 0.0 0.0 (Variables|Default|GetBlockOffset))) "0, 0, 0" "1.000000,1.000000,1.000000") "AlwaysSpawn" "MultiplyWithRoot" 0 0))
      (Transformation|AttachComponentToComponent _returnvalue (Utilities|Array|Get(acopy) (Variables|Default|GetSlots) _index) "None" "KeepWorld" "KeepWorld" "KeepWorld" true)
      (Variables|/Game/Blueprints/Puzzles/BridgePuzzle/BP_RaisedBridge.BP_RaisedBridge_C|SetbRaised (Utilities|Array|Get(acopy) (Variables|Default|GetBridges) _index) true)))
  (return))

(fn ShowUI
  (Utilities|IsValid (Variables|Default|GetCrosshairRef)
    (:Is%20Valid
      _)
    (:Is%20Not%20Valid
      (bind _returnvalue (UserInterface|CreateWidget "/Game/UI/WBP_Reticule.WBP_Reticule_C"))
      (bind _output_get (Variables|Default|SetCrosshairRef _returnvalue))))
  (UserInterface|Viewport|AddtoViewport _output_get 0)
  (Variables|/Game/ThirdPerson/Blueprints/BP_ThirdPersonCharacter.BP_ThirdPersonCharacter_C|SetbPanel (Variables|Default|GetPlayerRef) true)
  (return))

(fn RaiseBridge
  (for _index (range 0 (- (Utilities|Array|Length (Variables|Default|GetBridges)) 1))
    (if (Utilities|Array|Get(acopy) (Variables|Default|GetbFull) _index)
      (Variables|/Game/Blueprints/Puzzles/BridgePuzzle/BP_RaisedBridge.BP_RaisedBridge_C|SetbRaised (Utilities|Array|Get(acopy) (Variables|Default|GetBridges) _index) true)
      (else
        (Variables|/Game/Blueprints/Puzzles/BridgePuzzle/BP_RaisedBridge.BP_RaisedBridge_C|SetbRaised (Utilities|Array|Get(acopy) (Variables|Default|GetBridges) _index) false))))
  (return))

(fn CheckSlots
  (bind _bfull (Variables|Default|GetbFull))
  (for _index (range 0 (- (Utilities|Array|Length (Variables|Default|GetBridges)) 1))
    (Utilities|IsValid (Components|GetChildComponent (Utilities|Array|Get(acopy) (Variables|Default|GetSlots) _index) 0)
      (:Is%20Valid
        (Utilities|Array|SetArrayElem _bfull _index true))
      (:Is%20Not%20Valid
        (Utilities|Array|SetArrayElem _bfull _index false))))
  (CallFunction|RaiseBridge)
  (return))

(fn PlaceBlock
  (params (Slot :type Static%20Mesh%20Component%20Object%20Reference))
  (bind _playerref (Variables|Default|GetPlayerRef))
  (if (Variables|/Game/ThirdPerson/Blueprints/BP_ThirdPersonCharacter.BP_ThirdPersonCharacter_C|GetbCarrying (Variables|Default|GetPlayerRef))
    (bind _returnvalue (Game|SpawnActorfromClass "/Game/Blueprints/Puzzles/BridgePuzzle/BP_PuzzleKey.BP_PuzzleKey_C" (Math|Transform|MakeTransform (+ (Transformation|GetWorldLocation Slot) (Math|Vector|MakeVector 0.0 0.0 (Variables|Default|GetBlockOffset))) "0, 0, 0" "1.000000,1.000000,1.000000") "AlwaysSpawn" "MultiplyWithRoot" 0 0))
    (Transformation|AttachComponentToComponent _returnvalue Slot "None" "KeepWorld" "KeepWorld" "KeepWorld" true)
    (Actor|DestroyActor (Variables|/Game/ThirdPerson/Blueprints/BP_ThirdPersonCharacter.BP_ThirdPersonCharacter_C|GetCarriedBlock _playerref))
    (Variables|/Game/ThirdPerson/Blueprints/BP_ThirdPersonCharacter.BP_ThirdPersonCharacter_C|SetCarriedBlock _playerref 0)
    (Variables|/Game/ThirdPerson/Blueprints/BP_ThirdPersonCharacter.BP_ThirdPersonCharacter_C|SetbCarrying _playerref false)
    (return)
    (else
      (return))))

(fn HideUI
  (Utilities|IsValid (Variables|Default|GetCrosshairRef)
    (:Is%20Valid
      _)
    (:Is%20Not%20Valid
      (bind _returnvalue (UserInterface|CreateWidget "/Game/UI/WBP_Reticule.WBP_Reticule_C"))
      (bind _output_get (Variables|Default|SetCrosshairRef _returnvalue))))
  (Widget|RemovefromParent _output_get)
  (Variables|/Game/ThirdPerson/Blueprints/BP_ThirdPersonCharacter.BP_ThirdPersonCharacter_C|SetbPanel (Variables|Default|GetPlayerRef) false)
  (return))