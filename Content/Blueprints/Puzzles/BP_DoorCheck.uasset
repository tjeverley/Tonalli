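; BP_DoorCheck is a puzzle actor that records when the player passes a door check and restores its open state.
; When the player leaves the Trigger, it sets IsOpen and adds itself to OpenDoors in the player's inventory.
; Tick disables Trigger collision while IsOpen is true.
; BeginPlay caches the player character and, if already open, calls StartOpen to rotate the Ratchet's Spine, which the overlap itself never does.
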(event OnComponentEndOverlap(Trigger)
  (params (OverlappedComponent :type Primitive%20Component%20Object%20Reference) (OtherActor :type Actor%20Object%20Reference) (OtherComp :type Primitive%20Component%20Object%20Reference) (OtherBodyIndex :type Integer))
  (bind _playerref (Variables|Default|GetPlayerRef))
  (if (== OtherActor _playerref)
    (Variables|Default|SetbIsOpen true)
    (Utilities|Array|Add (Variables|/Game/ThirdPerson/Blueprints/BP_Inventory.BP_Inventory_C|GetOpenDoors (Variables|/Game/ThirdPerson/Blueprints/BP_ThirdPersonCharacter.BP_ThirdPersonCharacter_C|GetPlayerInventory _playerref)) self)))

(event EventBeginPlay
  (Utilities|IsValid (Variables|Default|GetPlayerRef)
    (:Is%20Valid
      _)
    (:Is%20Not%20Valid
      (bind _asbp_third_person_character (Utilities|Casting|CastToBP_ThirdPersonCharacter (Game|GetPlayerCharacter 0)))
      (Variables|Default|SetPlayerRef _asbp_third_person_character)))
  (if (Variables|Default|GetbIsOpen)
    (CallFunction|StartOpen)))

(event Collision|EventActorBeginOverlap
  (params (OtherActor :type Actor%20Object%20Reference)))

(event EventTick
  (params (DeltaSeconds :type Float%20%28single-precision%29))
  (if (Variables|Default|GetbIsOpen)
    (Collision|SetCollisionEnabled (Variables|Default|GetTrigger) "NoCollision")))

(fn ConstructionScript)

(fn StartOpen
  (Transformation|SetRelativeRotation (Variables|/Game/Blueprints/Puzzles/BP_RatchetSystem.BP_RatchetSystem_C|GetSpine (Variables|Default|GetRatchet)) "0.000000,180.000000,0.000000" false false)
  (return))