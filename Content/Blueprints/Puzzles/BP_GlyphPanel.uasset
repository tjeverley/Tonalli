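; Glyph panel puzzle with four buttons that depress, light up and each show their own output.
; An overlap volume toggles the reticle, prompt and player's Panel flag, optionally shows a tutorial, and resets unsolved puzzles on exit.
; Tick polls Value to press a glyph or play the reset timeline.
; CheckSolution, not called within this Blueprint, steps through the Solution array, setting Complete or restarting the sequence.
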(event OnComponentBeginOverlap(InteractionDetector)
  (params (OverlappedComponent :type Primitive%20Component%20Object%20Reference) (OtherActor :type Actor%20Object%20Reference) (OtherComp :type Primitive%20Component%20Object%20Reference) (OtherBodyIndex :type Integer) (bFromSweep :type Boolean) (SweepResult :type Hit%20Result%20Structure%20%28by%20ref%29))
  ;[0.15 0.15 0.15 0.5] Display/Hide Selection Cursor
  (Utilities|IsValid (Variables|Default|GetPlayerRef)
    (:Is%20Valid
      _)
    (:Is%20Not%20Valid
      (bind _asbp_third_person_character (Utilities|Casting|CastToBP_ThirdPersonCharacter (Game|GetPlayerCharacter 0)))
      (Variables|Default|SetPlayerRef _asbp_third_person_character)))
  (if (== OtherActor (Variables|Default|GetPlayerRef))
    (Utilities|IsValid (Variables|Default|GetCrosshairRef)
      (:Is%20Valid
        _)
      (:Is%20Not%20Valid
        (bind _returnvalue (UserInterface|CreateWidget "/Game/UI/WBP_Reticule.WBP_Reticule_C" (Game|GetPlayerController 0)))
        (bind _output_get (Variables|Default|SetCrosshairRef _returnvalue))))
    (UserInterface|Viewport|AddtoViewport _output_get 0)
    (Variables|/Game/ThirdPerson/Blueprints/BP_ThirdPersonCharacter.BP_ThirdPersonCharacter_C|SetbPanel (Variables|Default|GetPlayerRef) true)
    (Rendering|SetVisibility (Variables|Default|GetInteractionMessage) true false)
    ;[0.15 0.15 0.15 0.5] Tutorial
    (if (Variables|Default|GetbShowTurorial)
      (CallFunction|Tutorial))))

(event OnComponentEndOverlap(InteractionDetector)
  (params (OverlappedComponent :type Primitive%20Component%20Object%20Reference) (OtherActor :type Actor%20Object%20Reference) (OtherComp :type Primitive%20Component%20Object%20Reference) (OtherBodyIndex :type Integer))
  ;[0.15 0.15 0.15 0.5] Display/Hide Selection Cursor
  (Utilities|IsValid (Variables|Default|GetPlayerRef)
    (:Is%20Valid
      _)
    (:Is%20Not%20Valid
      (bind _asbp_third_person_character (Utilities|Casting|CastToBP_ThirdPersonCharacter (Game|GetPlayerCharacter 0)))
      (Variables|Default|SetPlayerRef _asbp_third_person_character)))
  (if (== OtherActor (Variables|Default|GetPlayerRef))
    (Utilities|IsValid (Variables|Default|GetCrosshairRef)
      (:Is%20Valid
        _)
      (:Is%20Not%20Valid
        (bind _returnvalue (UserInterface|CreateWidget "/Game/UI/WBP_Reticule.WBP_Reticule_C" (Game|GetPlayerController 0)))
        (bind _output_get (Variables|Default|SetCrosshairRef _returnvalue))))
    (Widget|RemovefromParent _output_get)
    (Variables|/Game/ThirdPerson/Blueprints/BP_ThirdPersonCharacter.BP_ThirdPersonCharacter_C|SetbPanel (Variables|Default|GetPlayerRef) false)
    (Rendering|SetVisibility (Variables|Default|GetInteractionMessage) false false)
    ;[0.15 0.15 0.15 0.5] Reset Puzzle if Not solved
    (if (not (Variables|Default|GetbComplete))
      (Variables|Default|SetValue 0))))

(event EventBeginPlay
  ;[0.15 0.15 0.15 0.5] Default
  (Variables|/Game/Blueprints/Tutorials/BP_Tutorial.BP_Tutorial_C|SetbDismissed (Variables|Default|GetBP_Tutorial) (not (Variables|Default|GetbShowTurorial)))
  (CallFunction|LightsOff)
  (Rendering|SetVisibility (Variables|Default|GetInteractionMessage) false false))

(event EventTick
  (params (DeltaSeconds :type Float%20%28single-precision%29))
  ;[0.15 0.15 0.15 0.5] Hide UI Once Solved
  (if (Variables|Default|GetbComplete)
    (Rendering|SetVisibility (Variables|Default|GetInteractionMessage) false false))
  ;[0.15 0.15 0.15 0.5] Take Input
  (switch int (Variables|Default|GetValue)
    (:0
      ;[0.15 0.15 0.15 0.5] Reset Panel
      (CallFunction|LightsOff)
      (bind _keysup (Timeline|ResetTimeline Play)
        (:Update
          ;;[0.15 0.15 0.15 0.5] Reset Glyph 1
          (Transformation|SetRelativeLocation (Variables|Default|GetGlyph1) (Math|Vector|MakeVector (Math|Float|Lerp -26.450218 -27.942728 _keysup) -80.274327 (Math|Float|Lerp 45.813122 49.91376 _keysup)) false false)
          ;;[0.15 0.15 0.15 0.5] Reset Glyph 2
          (Transformation|SetRelativeLocation (Variables|Default|GetGlyph2) (Math|Vector|MakeVector (Math|Float|Lerp -26.450218 -27.942728 _keysup) -26.65782 (Math|Float|Lerp 45.813122 49.91376 _keysup)) false false)
          ;;[0.15 0.15 0.15 0.5] Reset Glyph 3
          (Transformation|SetRelativeLocation (Variables|Default|GetGlyph3) (Math|Vector|MakeVector (Math|Float|Lerp -26.450218 -27.942728 _keysup) 28.382671 (Math|Float|Lerp 45.813122 49.91376 _keysup)) false false)
          (Transformation|SetRelativeLocation (Variables|Default|GetGlyph4) (Math|Vector|MakeVector (Math|Float|Lerp -26.450218 -27.942728 _keysup) 83.022278 (Math|Float|Lerp 45.813122 49.91376 _keysup)) false false)
          (Rendering|SetVisibility (Variables|Default|GetOutput1) false false)
          (Rendering|SetVisibility (Variables|Default|GetOutput2) false false)
          (Rendering|SetVisibility (Variables|Default|GetOutput3) false false)
          (Rendering|SetVisibility (Variables|Default|GetOutput4) false false))))
    (:1
      (Utilities|Depress1))
    (:2
      (Utilities|Depress2))
    (:3
      (Utilities|Depress3))
    (:4
      (Utilities|Depress4))))

(fn ConstructionScript)

(fn CheckSolution
  (params (Value :type Integer))
  ;[0.15 0.15 0.15 0.5] Check Value Against Solution
  (if (== Value (Utilities|Array|Get(acopy) (Variables|Default|GetSolution) (Variables|Default|GetSolutionIndex)))
    (if (== (Variables|Default|GetSolutionIndex) (- (Utilities|Array|Length (Variables|Default|GetSolution)) 1))
      ;[0.15 0.15 0.15 0.5] Mark Puzzle as Solved
      (Variables|Default|SetbComplete true)
      (else
        ;[0.15 0.15 0.15 0.5] Increment Index
        (Variables|Default|SetSolutionIndex (+ (Variables|Default|GetSolutionIndex) 1))))
    (else
      ;[0.15 0.15 0.15 0.5] Reset Puzzle
      (Variables|Default|SetValue 0)
      (Variables|Default|SetSolutionIndex 0)))
  (return))

(fn LightsOff
  (Rendering|Components|Light|SetIntensity (Variables|Default|GetConfirmLight1) 0.0)
  (Rendering|Components|Light|SetIntensity (Variables|Default|GetConfirmLight2) 0.0)
  (Rendering|Components|Light|SetIntensity (Variables|Default|GetConfirmLight3) 0.0)
  (Rendering|Components|Light|SetIntensity (Variables|Default|GetConfirmLight4) 0.0)
  (return))

(fn Tutorial
  (bind _bp_tutorial (Variables|Default|GetBP_Tutorial))
  (Variables|/Game/ThirdPerson/Blueprints/BP_ThirdPersonCharacter.BP_ThirdPersonCharacter_C|SetbDialogue (Variables|Default|GetPlayerRef) true)
  (if (Variables|/Game/Blueprints/Tutorials/BP_Tutorial.BP_Tutorial_C|GetbDismissed _bp_tutorial)
    (return)
    (else
      (Default|ShowTutorial _bp_tutorial)
      (Default|DialogueBox (Variables|Default|GetPlayerRef))
      (Variables|/Game/Blueprints/Tutorials/BP_Tutorial.BP_Tutorial_C|SetbDismissed (Variables|Default|GetBP_Tutorial) true)
      (return))))