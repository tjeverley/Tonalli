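; BP_RotationPuzzle is a three-ring rotation puzzle that slides its rings away once all are solved.
; BeginPlay sets starting yaw for CoreRing and Ring1 only; Rotate offsets a ring's yaw and returns whether its rounded value matches the solution.
; Tick polls the three solved flags, disables ring collision, then runs delay-chained timelines lowering Ring2, Ring1 and CoreRing in turn before sliding all three along X.
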(event EventBeginPlay
  (bind _corering (Variables|Default|GetCoreRing))
  (bind _ring1 (Variables|Default|GetRing1))
  (bind _relativerotation (Variables|/Script/Engine.SceneComponent|GetRelativeRotation _ring1))
  (bind _relativerotation_2 (Variables|/Script/Engine.SceneComponent|GetRelativeRotation _corering))
  ;[0.15 0.15 0.15 0.5] Set Starting Angle
  (Transformation|SetRelativeRotation _corering (Math|Rotator|MakeRotator (.roll _relativerotation_2) (.pitch _relativerotation_2) (Variables|Default|GetCore_StartingAngle)) false false)
  (Transformation|SetRelativeRotation _ring1 (Math|Rotator|MakeRotator (.roll _relativerotation) (.pitch _relativerotation) (Variables|Default|GetRing1_StartingAngle)) false false))

(event Collision|EventActorBeginOverlap
  (params (OtherActor :type Actor%20Object%20Reference)))

(event EventTick
  (params (DeltaSeconds :type Float%20%28single-precision%29))
  (bind _ring1 (Variables|Default|GetRing1))
  (bind _corering (Variables|Default|GetCoreRing))
  (bind _corering_2 (Variables|Default|GetCoreRing))
  (bind _ring1_2 (Variables|Default|GetRing1))
  (bind _ring2 (Variables|Default|GetRing2))
  (bind _ring2_2 (Variables|Default|GetRing2))
  (bind _relativelocation (Variables|/Script/Engine.SceneComponent|GetRelativeLocation _corering))
  (bind _relativelocation_2 (Variables|/Script/Engine.SceneComponent|GetRelativeLocation _ring2_2))
  (bind _relativelocation_3 (Variables|/Script/Engine.SceneComponent|GetRelativeLocation _corering_2))
  (bind _relativelocation_4 (Variables|/Script/Engine.SceneComponent|GetRelativeLocation _ring2))
  (bind _relativelocation_5 (Variables|/Script/Engine.SceneComponent|GetRelativeLocation _ring1_2))
  (bind _relativelocation_6 (Variables|/Script/Engine.SceneComponent|GetRelativeLocation _ring1))
  (if (Math|Boolean|ANDBoolean (Variables|Default|GetCore_Solved) (Variables|Default|GetRing1_Solved) (Variables|Default|GetRing2_Solved))
    (Collision|SetCollisionEnabled (Variables|Default|GetCoreRing) "NoCollision")
    (bind _movement (Timeline|Unlock Play)
      (:Update
        (Transformation|SetRelativeLocation _ring2_2 (Math|Vector|MakeVector (.x _relativelocation_2) (.y _relativelocation_2) (Math|Float|Lerp 0.0 -2e+01 _movement)) false false))
      (:Finished
        (Utilities|FlowControl|Delay 1.0)
        (bind _movement_2 (Timeline|Timeline_0 Play)
          (:Update
            (Transformation|SetRelativeLocation _ring1 (Math|Vector|MakeVector (.x _relativelocation_6) (.y _relativelocation_6) (Math|Float|Lerp 0.0 -2e+01 _movement_2)) false false))
          (:Finished
            (Utilities|FlowControl|Delay 1.0)
            (bind _movement_3 (Timeline|Timeline Play)
              (:Update
                (Transformation|SetRelativeLocation _corering (Math|Vector|MakeVector (.x _relativelocation) (.y _relativelocation) (Math|Float|Lerp 0.0 -2e+01 _movement_3)) false false))
              (:Finished
                (Utilities|FlowControl|Delay 1.0)
                (bind _open (Timeline|RevealSecret Play)
                  (:Update
                    (Transformation|SetRelativeLocation _ring2 (Math|Vector|MakeVector (Math|Float|Lerp 0.0 -1.5e+02 _open) (.y _relativelocation_4) (.z _relativelocation_4)) false false)
                    (Transformation|SetRelativeLocation _ring1_2 (Math|Vector|MakeVector (Math|Float|Lerp 0.0 -1.5e+02 _open) (.y _relativelocation_5) (.z _relativelocation_5)) false false)
                    (Transformation|SetRelativeLocation _corering_2 (Math|Vector|MakeVector (Math|Float|Lerp 0.0 -1.5e+02 _open) (.y _relativelocation_3) (.z _relativelocation_3)) false false)))))))))))

(fn ConstructionScript)

(fn Rotate
  (params (Angle :type Float%20%28double-precision%29) (RotatedMesh :type Static%20Mesh%20Component%20Object%20Reference) (StartingAngle :type Float%20%28double-precision%29) (Solution :type Float%20%28double-precision%29))
  (bind _relativerotation (Variables|/Script/Engine.SceneComponent|GetRelativeRotation RotatedMesh))
  ;[0.15 0.15 0.15 0.5] Update Rotation Angle
  (Transformation|SetRelativeRotation RotatedMesh (Math|Rotator|MakeRotator (.roll _relativerotation) (.pitch _relativerotation) (+ StartingAngle Angle)) false false)
  (if (== (Class|KismetMathLibrary|Round64 (.yaw _relativerotation)) Solution)
    (return true)
    (else
      (return false))))