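; Puzzle bowl where the player gives up a Stone Heart to unlock a linked Barricade, whose Direction it sets on BeginPlay.
; InteractionDetector overlaps show a prompt, turned toward the camera on entry, and enable interaction if the inventory holds a heart.
; Tick polls the player's Interaction flag, then slots the Heart mesh into place, unlocks the Barricade and deducts one heart, once only.
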(event OnComponentBeginOverlap(InteractionDetector)
  (params (OverlappedComponent :type Primitive%20Component%20Object%20Reference) (OtherActor :type Actor%20Object%20Reference) (OtherComp :type Primitive%20Component%20Object%20Reference) (OtherBodyIndex :type Integer) (bFromSweep :type Boolean) (SweepResult :type Hit%20Result%20Structure%20%28by%20ref%29))
  ;[0.15 0.15 0.15 0.5] Display/Hiude UI
  (Utilities|IsValid (Variables|Default|GetPlayerRef)
    (:Is%20Valid
      _)
    (:Is%20Not%20Valid
      (bind _asbp_third_person_character (Utilities|Casting|CastToBP_ThirdPersonCharacter OtherActor))
      (Variables|Default|SetPlayerRef _asbp_third_person_character)))
  (bind _haskey (CallFunction|CheckforHeart))
  (if (and _haskey (not (Variables|Default|GetbUnlocked)))
    (CallFunction|WidgetFacePlayer)
    (Rendering|SetVisibility (Variables|Default|GetInteractionMessage) true false)
    (Variables|Default|SetbCanInteract true)))

(event OnComponentEndOverlap(InteractionDetector)
  (params (OverlappedComponent :type Primitive%20Component%20Object%20Reference) (OtherActor :type Actor%20Object%20Reference) (OtherComp :type Primitive%20Component%20Object%20Reference) (OtherBodyIndex :type Integer))
  ;[0.15 0.15 0.15 0.5] Display/Hiude UI
  (Utilities|IsValid (Variables|Default|GetPlayerRef)
    (:Is%20Valid
      _)
    (:Is%20Not%20Valid
      (bind _asbp_third_person_character (Utilities|Casting|CastToBP_ThirdPersonCharacter OtherActor))
      (Variables|Default|SetPlayerRef _asbp_third_person_character)))
  (if (not (Variables|Default|GetbUnlocked))
    (Rendering|SetVisibility (Variables|Default|GetInteractionMessage) false false)
    (Variables|Default|SetbCanInteract false)))

(event EventBeginPlay
  (bind _barricade (Variables|Default|GetBarricade))
  ;[0.15 0.15 0.15 0.5] Set Barrier Direction
  (Utilities|IsValid _barricade
    (:Is%20Valid
      (Variables|/Game/Blueprints/Puzzles/BP_SacrificeBarrier.BP_SacrificeBarrier_C|SetDirection _barricade (Variables|Default|GetDirection)))))

(event Collision|EventActorBeginOverlap
  (params (OtherActor :type Actor%20Object%20Reference)))

(event EventTick
  (params (DeltaSeconds :type Float%20%28single-precision%29))
  (bind _heart (Variables|Default|GetHeart))
  ;[0.15 0.15 0.15 0.5] Get Player
  (Utilities|IsValid (Variables|Default|GetPlayerRef)
    (:Is%20Valid
      _)
    (:Is%20Not%20Valid
      (bind _asbp_third_person_character (Utilities|Casting|CastToBP_ThirdPersonCharacter (Game|GetPlayerCharacter 0)))
      (bind _output_get (Variables|Default|SetPlayerRef _asbp_third_person_character))))
  ;[0.15 0.15 0.15 0.5] Check for Interaction
  (if (and (Variables|Default|GetbCanInteract) (Variables|/Game/ThirdPerson/Blueprints/BP_ThirdPersonCharacter.BP_ThirdPersonCharacter_C|GetbInteraction _output_get))
    (if (not (Variables|Default|GetbUnlocked))
      ;[0.15 0.15 0.15 0.5] Slot Heart Into Place
      (Variables|Default|SetbUnlocked true)
      (Rendering|SetVisibility _heart true false)
      (Components|MoveComponentTo _heart "0.000000,0.000000,50.000000" "0, 0, 0" false false 1.0 false)
      (Variables|/Game/Blueprints/Puzzles/BP_SacrificeBarrier.BP_SacrificeBarrier_C|SetbUnlocked (Variables|Default|GetBarricade) true)
      ;[0.15 0.15 0.15 0.5] Remove Heart From Inventory
      (Variables|/Game/ThirdPerson/Blueprints/BP_Inventory.BP_Inventory_C|SetStoneHearts (Variables|/Game/ThirdPerson/Blueprints/BP_ThirdPersonCharacter.BP_ThirdPersonCharacter_C|GetPlayerInventory (Variables|Default|GetPlayerRef)) (- (Variables|/Game/ThirdPerson/Blueprints/BP_Inventory.BP_Inventory_C|GetStoneHearts (Variables|/Game/ThirdPerson/Blueprints/BP_ThirdPersonCharacter.BP_ThirdPersonCharacter_C|GetPlayerInventory (Variables|Default|GetPlayerRef))) 1)))))

(fn ConstructionScript)

(fn WidgetFacePlayer
  ;[0.15 0.15 0.15 0.5] Orient UI to Face Player
  (Transformation|SetWorldRotation (Variables|Default|GetInteractionMessage) (Math|Rotator|FindLookatRotation (Transformation|GetWorldLocation (Variables|Default|GetInteractionMessage)) (Transformation|GetWorldLocation (Variables|/Script/Engine.PlayerCameraManager|GetTransformComponent (Game|GetPlayerCameraManager 0)))) false false)
  (return))

(fn CheckforHeart
  (Utilities|IsValid (Variables|Default|GetPlayerRef)
    (:Is%20Valid
      _)
    (:Is%20Not%20Valid
      (bind _asbp_third_person_character (Utilities|Casting|CastToBP_ThirdPersonCharacter (Game|GetPlayerCharacter 0)))
      (bind _output_get (Variables|Default|SetPlayerRef _asbp_third_person_character))))
  (if (> (Variables|/Game/ThirdPerson/Blueprints/BP_Inventory.BP_Inventory_C|GetStoneHearts (Variables|/Game/ThirdPerson/Blueprints/BP_ThirdPersonCharacter.BP_ThirdPersonCharacter_C|GetPlayerInventory _output_get)) 0)
    (return true)
    (else
      (return false))))