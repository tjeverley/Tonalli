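; Cog wall puzzle where the player places carried cogs on three spindles in the correct order.
; An overlap zone shows slot prompts and a reticle, enables the player's line casting, and can trigger a one-time tutorial.
; Per-slot load and unload functions attach cogs to spindles or return them to the player.
; Once all slots are filled, Tick compares gear IDs with the Solution array and sets Complete on a match.
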(event OnComponentBeginOverlap(InteractionDetector)
  (params (OverlappedComponent :type Primitive%20Component%20Object%20Reference) (OtherActor :type Actor%20Object%20Reference) (OtherComp :type Primitive%20Component%20Object%20Reference) (OtherBodyIndex :type Integer) (bFromSweep :type Boolean) (SweepResult :type Hit%20Result%20Structure%20%28by%20ref%29))
  ;[0.15 0.15 0.15 0.5] Spindle Access
  (Utilities|IsValid (Variables|Default|GetPlayerRef)
    (:Is%20Valid
      _)
    (:Is%20Not%20Valid
      (bind _asbp_third_person_character (Utilities|Casting|CastToBP_ThirdPersonCharacter (Game|GetPlayerCharacter 0)))
      (Variables|Default|SetPlayerRef _asbp_third_person_character)))
  (if (== OtherActor (Variables|Default|GetPlayerRef))
    (if (not (Variables|Default|GetbComplete))
      (Variables|Default|SetbCanInteract true)
      ;[0.15 0.15 0.15 0.5] Display/Hide UI
      (CallFunction|ShowUI)
      ;[0.15 0.15 0.15 0.5] Tutorial
      (if (Variables|Default|GetbShowTutorial)
        (CallFunction|Tutorial)))))

(event OnComponentEndOverlap(InteractionDetector)
  (params (OverlappedComponent :type Primitive%20Component%20Object%20Reference) (OtherActor :type Actor%20Object%20Reference) (OtherComp :type Primitive%20Component%20Object%20Reference) (OtherBodyIndex :type Integer))
  ;[0.15 0.15 0.15 0.5] Spindle Access
  (Utilities|IsValid (Variables|Default|GetPlayerRef)
    (:Is%20Valid
      _)
    (:Is%20Not%20Valid
      (bind _asbp_third_person_character (Utilities|Casting|CastToBP_ThirdPersonCharacter (Game|GetPlayerCharacter 0)))
      (Variables|Default|SetPlayerRef _asbp_third_person_character)))
  (if (== OtherActor (Variables|Default|GetPlayerRef))
    (Variables|Default|SetbCanInteract false)
    ;[0.15 0.15 0.15 0.5] Display/Hide UI
    (CallFunction|HideUI)))

(event EventBeginPlay
  (Variables|/Game/Blueprints/Tutorials/BP_Tutorial.BP_Tutorial_C|SetbDismissed (Variables|Default|GetBP_Tutorial) (not (Variables|Default|GetbShowTutorial)))
  (CallFunction|HideUI))

(event Collision|EventActorBeginOverlap
  (params (OtherActor :type Actor%20Object%20Reference)))

(event EventTick
  (params (DeltaSeconds :type Float%20%28single-precision%29))
  (if (Math|Boolean|ANDBoolean (Variables|Default|GetbLoadedA) (Variables|Default|GetbLoadedB) (Variables|Default|GetbLoadedC))
    (CallFunction|CheckSolution)))

(fn ConstructionScript)

(fn HideUI
  ;[0.15 0.15 0.15 0.5] Hide Interaction Messages
  (Rendering|SetVisibility (Variables|Default|GetSlotA_FullMessage) false false)
  (Rendering|SetVisibility (Variables|Default|GetSlotA_EmptyMessage) false false)
  (Rendering|SetVisibility (Variables|Default|GetSlotB_FullMessage) false false)
  (Rendering|SetVisibility (Variables|Default|GetSlotB_EmptyMessage) false false)
  (Rendering|SetVisibility (Variables|Default|GetSlotC_FullMessage) false false)
  (Rendering|SetVisibility (Variables|Default|GetSlotC_EmptyMessage) false false)
  ;[0.15 0.15 0.15 0.5] Hide Crosshair
  (Utilities|IsValid (Variables|Default|GetCrosshairRef)
    (:Is%20Valid
      _)
    (:Is%20Not%20Valid
      (bind _returnvalue (UserInterface|CreateWidget "/Game/UI/WBP_Reticule.WBP_Reticule_C"))
      (bind _output_get (Variables|Default|SetCrosshairRef _returnvalue))))
  (Widget|RemovefromParent _output_get)
  ;[0.15 0.15 0.15 0.5] Stop Line Casting
  (Utilities|IsValid (Variables|Default|GetPlayerRef)
    (:Is%20Valid
      _)
    (:Is%20Not%20Valid
      (bind _asbp_third_person_character (Utilities|Casting|CastToBP_ThirdPersonCharacter (Game|GetPlayerCharacter 0)))
      (bind _output_get_2 (Variables|Default|SetPlayerRef _asbp_third_person_character))))
  (Variables|/Game/ThirdPerson/Blueprints/BP_ThirdPersonCharacter.BP_ThirdPersonCharacter_C|SetbPanel _output_get_2 false)
  (return))

(fn ShowUI
  ;[0.15 0.15 0.15 0.5] If Player is Carrying Cog
  (Utilities|IsValid (Variables|Default|GetPlayerRef)
    (:Is%20Valid
      _)
    (:Is%20Not%20Valid
      (bind _asbp_third_person_character (Utilities|Casting|CastToBP_ThirdPersonCharacter (Game|GetPlayerCharacter 0)))
      (bind _output_get (Variables|Default|SetPlayerRef _asbp_third_person_character))))
  (LocalVariables|SetbIsCarrying (Variables|/Game/ThirdPerson/Blueprints/BP_ThirdPersonCharacter.BP_ThirdPersonCharacter_C|GetbCarrying _output_get))
  ;[0.15 0.15 0.15 0.5] Slot 1
  (if (Variables|Default|GetbLoadedA)
    (Rendering|SetVisibility (Variables|Default|GetSlotA_FullMessage) true false)
    (elif (LocalVariables|GetbIsCarrying)
      (Rendering|SetVisibility (Variables|Default|GetSlotA_EmptyMessage) true false)))
  ;[0.15 0.15 0.15 0.5] Slot 2
  (if (Variables|Default|GetbLoadedB)
    (Rendering|SetVisibility (Variables|Default|GetSlotB_FullMessage) true false)
    (elif (LocalVariables|GetbIsCarrying)
      (Rendering|SetVisibility (Variables|Default|GetSlotB_EmptyMessage) true false)))
  ;[0.15 0.15 0.15 0.5] Slot 3
  (if (Variables|Default|GetbLoadedC)
    (Rendering|SetVisibility (Variables|Default|GetSlotC_FullMessage) true false)
    (elif (LocalVariables|GetbIsCarrying)
      (Rendering|SetVisibility (Variables|Default|GetSlotC_EmptyMessage) true false)))
  ;[0.15 0.15 0.15 0.5] Show Crosshair
  (Utilities|IsValid (Variables|Default|GetCrosshairRef)
    (:Is%20Valid
      _)
    (:Is%20Not%20Valid
      (bind _returnvalue (UserInterface|CreateWidget "/Game/UI/WBP_Reticule.WBP_Reticule_C"))
      (bind _output_get_2 (Variables|Default|SetCrosshairRef _returnvalue))))
  (UserInterface|Viewport|AddtoViewport _output_get_2 0)
  (Variables|/Game/ThirdPerson/Blueprints/BP_ThirdPersonCharacter.BP_ThirdPersonCharacter_C|SetbPanel (Variables|Default|GetPlayerRef) true)
  (return))

(fn PlaceCog
  (params (SlotLocation :type Vector))
  ;[0.15 0.15 0.15 0.5] Get Desired Slot Coordinates
  (LocalVariables|SetSlot SlotLocation)
  ;[0.15 0.15 0.15 0.5] Get Carried Cog
  (Utilities|IsValid (Variables|Default|GetPlayerRef)
    (:Is%20Valid
      _)
    (:Is%20Not%20Valid
      (bind _asbp_third_person_character (Utilities|Casting|CastToBP_ThirdPersonCharacter (Game|GetPlayerCharacter 0)))
      (bind _output_get (Variables|Default|SetPlayerRef _asbp_third_person_character))))
  ;[0.15 0.15 0.15 0.5] Detach Cog From Player
  (Transformation|DetachFromActor (Variables|/Game/ThirdPerson/Blueprints/BP_ThirdPersonCharacter.BP_ThirdPersonCharacter_C|GetCarriedItem _output_get) "KeepWorld" "KeepWorld" "KeepWorld")
  (Variables|/Game/ThirdPerson/Blueprints/BP_ThirdPersonCharacter.BP_ThirdPersonCharacter_C|SetbCarrying _output_get false)
  ;[0.15 0.15 0.15 0.5] Attach Cog To Spindle
  (bind _returnvalue (Transformation|AttachActorToActor (Variables|/Game/ThirdPerson/Blueprints/BP_ThirdPersonCharacter.BP_ThirdPersonCharacter_C|GetCarriedItem _output_get) self "None" "SnapToTarget" "SnapToTarget" "SnapToTarget" true))
  (LocalVariables|SetbLoaded _returnvalue)
  ;[0.15 0.15 0.15 0.5] Set Cog Orientation
  (Transformation|SetRelativeLocation (Variables|/Game/Blueprints/Puzzles/BP_Cog.BP_Cog_C|GetGearMesh (Variables|/Game/ThirdPerson/Blueprints/BP_ThirdPersonCharacter.BP_ThirdPersonCharacter_C|GetCarriedItem _output_get)) (LocalVariables|GetSlot) false false)
  (Transformation|SetRelativeRotation (Variables|/Game/Blueprints/Puzzles/BP_Cog.BP_Cog_C|GetGearMesh (Variables|/Game/ThirdPerson/Blueprints/BP_ThirdPersonCharacter.BP_ThirdPersonCharacter_C|GetCarriedItem _output_get)) "0.000000,90.000000,0.000000" false false)
  (return (LocalVariables|GetbLoaded) (Variables|/Game/ThirdPerson/Blueprints/BP_ThirdPersonCharacter.BP_ThirdPersonCharacter_C|GetCarriedItem _output_get)))

(fn LoadSlot1
  (bind _spindle_left (Variables|Default|GetSpindle_Left))
  (bind _relativelocation (Variables|/Script/Engine.SceneComponent|GetRelativeLocation _spindle_left))
  (bind (_loadstatus _placedcog) (CallFunction|PlaceCog (Math|Vector|MakeVector (+ (Variables|Default|GetGearOffset) (.x _relativelocation)) (.y _relativelocation) (.z _relativelocation))))
  (Variables|Default|SetbLoadedA _loadstatus)
  (Variables|Default|SetGear1 _placedcog)
  (Rendering|SetVisibility (Variables|Default|GetSlotA_EmptyMessage) false false)
  (Rendering|SetVisibility (Variables|Default|GetSlotA_FullMessage) true false)
  (return))

(fn LoadSlot2
  (bind _spindle_middle (Variables|Default|GetSpindle_Middle))
  (bind _relativelocation (Variables|/Script/Engine.SceneComponent|GetRelativeLocation _spindle_middle))
  (bind (_loadstatus _placedcog) (CallFunction|PlaceCog (Math|Vector|MakeVector (+ (Variables|Default|GetGearOffset) (.x _relativelocation)) (.y _relativelocation) (.z _relativelocation))))
  (Variables|Default|SetbLoadedB _loadstatus)
  (Variables|Default|SetGear2 _placedcog)
  (Rendering|SetVisibility (Variables|Default|GetSlotB_EmptyMessage) false false)
  (Rendering|SetVisibility (Variables|Default|GetSlotB_FullMessage) true false)
  (return))

(fn LoadSlot3
  (bind _spindle_right (Variables|Default|GetSpindle_Right))
  (bind _relativelocation (Variables|/Script/Engine.SceneComponent|GetRelativeLocation _spindle_right))
  (bind (_loadstatus _placedcog) (CallFunction|PlaceCog (Math|Vector|MakeVector (+ (Variables|Default|GetGearOffset) (.x _relativelocation)) (.y _relativelocation) (.z _relativelocation))))
  (Variables|Default|SetbLoadedC _loadstatus)
  (Variables|Default|SetGear3 _placedcog)
  (Rendering|SetVisibility (Variables|Default|GetSlotC_EmptyMessage) false false)
  (Rendering|SetVisibility (Variables|Default|GetSlotC_FullMessage) true false)
  (return))

(fn UnloadSlot1
  ;[0.15 0.15 0.15 0.5] Check If Player Already Has Cog
  (Utilities|IsValid (Variables|Default|GetPlayerRef)
    (:Is%20Valid
      _)
    (:Is%20Not%20Valid
      (bind _asbp_third_person_character (Utilities|Casting|CastToBP_ThirdPersonCharacter (Game|GetPlayerCharacter 0)))
      (bind _output_get (Variables|Default|SetPlayerRef _asbp_third_person_character))))
  (if (Variables|/Game/ThirdPerson/Blueprints/BP_ThirdPersonCharacter.BP_ThirdPersonCharacter_C|GetbCarrying _output_get)
    (Default|DropCog (Variables|/Game/ThirdPerson/Blueprints/BP_ThirdPersonCharacter.BP_ThirdPersonCharacter_C|GetCarriedItem (Variables|Default|GetPlayerRef))))
  (Transformation|DetachFromActor (Variables|Default|GetGear1) "KeepWorld" "KeepWorld" "KeepWorld")
  (Default|PickUpCog (Variables|Default|GetGear1))
  (Variables|Default|SetGear1 0)
  (Rendering|SetVisibility (Variables|Default|GetSlotA_EmptyMessage) true false)
  (Rendering|SetVisibility (Variables|Default|GetSlotA_FullMessage) false false)
  (Variables|Default|SetbLoadedA false)
  (return))

(fn UnloadSlot2
  ;[0.15 0.15 0.15 0.5] Check If Player Already Has Cog
  (Utilities|IsValid (Variables|Default|GetPlayerRef)
    (:Is%20Valid
      _)
    (:Is%20Not%20Valid
      (bind _asbp_third_person_character (Utilities|Casting|CastToBP_ThirdPersonCharacter (Game|GetPlayerCharacter 0)))
      (bind _output_get (Variables|Default|SetPlayerRef _asbp_third_person_character))))
  (if (Variables|/Game/ThirdPerson/Blueprints/BP_ThirdPersonCharacter.BP_ThirdPersonCharacter_C|GetbCarrying _output_get)
    (Default|DropCog (Variables|/Game/ThirdPerson/Blueprints/BP_ThirdPersonCharacter.BP_ThirdPersonCharacter_C|GetCarriedItem (Variables|Default|GetPlayerRef))))
  (Transformation|DetachFromActor (Variables|Default|GetGear2) "KeepWorld" "KeepWorld" "KeepWorld")
  (Default|PickUpCog (Variables|Default|GetGear2))
  (Variables|Default|SetGear2 0)
  (Rendering|SetVisibility (Variables|Default|GetSlotB_EmptyMessage) true false)
  (Rendering|SetVisibility (Variables|Default|GetSlotB_FullMessage) false false)
  (Variables|Default|SetbLoadedB false)
  (return))

(fn UnloadSlot3
  ;[0.15 0.15 0.15 0.5] Check If Player Already Has Cog
  (Utilities|IsValid (Variables|Default|GetPlayerRef)
    (:Is%20Valid
      _)
    (:Is%20Not%20Valid
      (bind _asbp_third_person_character (Utilities|Casting|CastToBP_ThirdPersonCharacter (Game|GetPlayerCharacter 0)))
      (bind _output_get (Variables|Default|SetPlayerRef _asbp_third_person_character))))
  (if (Variables|/Game/ThirdPerson/Blueprints/BP_ThirdPersonCharacter.BP_ThirdPersonCharacter_C|GetbCarrying _output_get)
    (Default|DropCog (Variables|/Game/ThirdPerson/Blueprints/BP_ThirdPersonCharacter.BP_ThirdPersonCharacter_C|GetCarriedItem (Variables|Default|GetPlayerRef))))
  (Transformation|DetachFromActor (Variables|Default|GetGear3) "KeepWorld" "KeepWorld" "KeepWorld")
  (Default|PickUpCog (Variables|Default|GetGear3))
  (Variables|Default|SetGear3 0)
  (Rendering|SetVisibility (Variables|Default|GetSlotB_EmptyMessage) true false)
  (Rendering|SetVisibility (Variables|Default|GetSlotB_FullMessage) false false)
  (Variables|Default|SetbLoadedC false)
  (return))

(fn CheckSolution
  ;[0.15 0.15 0.15 0.5] Set Puzzle as Completed
  (if (Math|Boolean|ANDBoolean (== (Utilities|Array|Get(acopy) (Variables|Default|GetSolution)) (Variables|/Game/Blueprints/Puzzles/BP_Cog.BP_Cog_C|GetID (Variables|Default|GetGear1))) (== (Utilities|Array|Get(acopy) (Variables|Default|GetSolution) 1) (Variables|/Game/Blueprints/Puzzles/BP_Cog.BP_Cog_C|GetID (Variables|Default|GetGear2))) (== (Utilities|Array|Get(acopy) (Variables|Default|GetSolution) 2) (Variables|/Game/Blueprints/Puzzles/BP_Cog.BP_Cog_C|GetID (Variables|Default|GetGear3))))
    (Variables|Default|SetbComplete true))
  (return))

(fn Tutorial
  (bind _bp_tutorial (Variables|Default|GetBP_Tutorial))
  (Variables|/Game/ThirdPerson/Blueprints/BP_ThirdPersonCharacter.BP_ThirdPersonCharacter_C|SetbDialogue (Variables|Default|GetPlayerRef) true)
  (if (Variables|/Game/Blueprints/Tutorials/BP_Tutorial.BP_Tutorial_C|GetbDismissed _bp_tutorial)
    (return)
    (else
      (Default|ShowTutorial _bp_tutorial)
      (Default|DialogueBox (Variables|Default|GetPlayerRef))
      (Variables|/Game/Blueprints/Tutorials/BP_Tutorial.BP_Tutorial_C|SetbDismissed (Variables|Default|GetBP_Tutorial) true)
      (return))))