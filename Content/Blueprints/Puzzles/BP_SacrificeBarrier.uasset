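; Puzzle barrier that slides its Cube mesh by a set Distance along a chosen axis once Unlocked is true.
; BeginPlay applies the configurable Mesh to the Cube; nothing in this graph sets Unlocked.
; Tick switches on Direction and calls a two-second MoveComponentTo toward the negative side of that axis.
; The target derives from the current location and Unlocked is never cleared here, so the move is reissued while unlocked.
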(event EventBeginPlay
  (Components|StaticMesh|SetStaticMesh (Variables|Default|GetCube) (Variables|Default|GetMesh)))

(event Collision|EventActorBeginOverlap
  (params (OtherActor :type Actor%20Object%20Reference)))

(event EventTick
  (params (DeltaSeconds :type Float%20%28single-precision%29))
  (bind _cube (Variables|Default|GetCube))
  (bind _cube_2 (Variables|Default|GetCube))
  (bind _cube_3 (Variables|Default|GetCube))
  (bind _relativelocation (Variables|/Script/Engine.SceneComponent|GetRelativeLocation _cube_3))
  (bind _relativelocation_2 (Variables|/Script/Engine.SceneComponent|GetRelativeLocation _cube_2))
  (bind _relativerotation (Variables|/Script/Engine.SceneComponent|GetRelativeRotation _cube))
  (bind _relativelocation_3 (Variables|/Script/Engine.SceneComponent|GetRelativeLocation _cube))
  (if (Variables|Default|GetbUnlocked)
    (switch Utilities|FlowControl|Switch|SwitchonBP_EnumAxes (Variables|Default|GetDirection)
      (:NewEnumerator0
        (Components|MoveComponentTo _cube (Math|Vector|MakeVector (- (.x _relativelocation_3) (Variables|Default|GetDistance)) (.y _relativelocation_3) (.z _relativelocation_3)) _relativerotation false false 2.0 false))
      (:NewEnumerator1
        (Components|MoveComponentTo _cube_2 (Math|Vector|MakeVector (.x _relativelocation_2) (- (.y _relativelocation_2) (Variables|Default|GetDistance)) (.z _relativelocation_2)) _relativerotation false false 2.0 false))
      (:NewEnumerator2
        (Components|MoveComponentTo _cube_3 (Math|Vector|MakeVector (.x _relativelocation) (.y _relativelocation) (- (.z _relativelocation) (Variables|Default|GetDistance))) _relativerotation false false 2.0 false)))))

(fn ConstructionScript)