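; Health pickup that adds one health item to the third-person character's inventory, then destroys itself.
; Overlapping InteractionDetector caches the player, enables interaction and shows a prompt widget, rotated once toward the camera.
; Tick polls the player's Interaction flag to trigger collection.
; End overlap hides the prompt and disables interaction only when the cached player is invalid, so both normally persist after the player leaves.
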(event OnComponentBeginOverlap(InteractionDetector)
  (params (OverlappedComponent :type Primitive%20Component%20Object%20Reference) (OtherActor :type Actor%20Object%20Reference) (OtherComp :type Primitive%20Component%20Object%20Reference) (OtherBodyIndex :type Integer) (bFromSweep :type Boolean) (SweepResult :type Hit%20Result%20Structure%20%28by%20ref%29))
  ;[0.15 0.15 0.15 0.5] Display/Hide UI
  (Utilities|IsValid (Variables|Default|GetPlayerRef)
    (:Is%20Valid
      _)
    (:Is%20Not%20Valid
      (bind _asbp_third_person_character (Utilities|Casting|CastToBP_ThirdPersonCharacter OtherActor))
      (Variables|Default|SetPlayerRef _asbp_third_person_character)))
  (CallFunction|WidgetFacePlayer)
  (Rendering|SetVisibility (Variables|Default|GetPickUpMessage) true false)
  (Variables|Default|SetbCanInteract true))

(event OnComponentEndOverlap(InteractionDetector)
  (params (OverlappedComponent :type Primitive%20Component%20Object%20Reference) (OtherActor :type Actor%20Object%20Reference) (OtherComp :type Primitive%20Component%20Object%20Reference) (OtherBodyIndex :type Integer))
  ;[0.15 0.15 0.15 0.5] Display/Hide UI
  (Utilities|IsValid (Variables|Default|GetPlayerRef)
    (:Is%20Not%20Valid
      (bind _asbp_third_person_character (Utilities|Casting|CastToBP_ThirdPersonCharacter OtherActor))
      (Variables|Default|SetPlayerRef _asbp_third_person_character)
      (Rendering|SetVisibility (Variables|Default|GetPickUpMessage) false false)
      (Variables|Default|SetbCanInteract false))))

(event EventBeginPlay
  ;[0.15 0.15 0.15 0.5] Default Values
  (Rendering|SetVisibility (Variables|Default|GetPickUpMessage) false false))

(event Collision|EventActorBeginOverlap
  (params (OtherActor :type Actor%20Object%20Reference)))

(event EventTick
  (params (DeltaSeconds :type Float%20%28single-precision%29))
  ;[0.15 0.15 0.15 0.5] Pick Up Key
  (Utilities|IsValid (Variables|Default|GetPlayerRef)
    (:Is%20Valid
      _)
    (:Is%20Not%20Valid
      (bind _asbp_third_person_character (Utilities|Casting|CastToBP_ThirdPersonCharacter (Variables|Default|GetPlayerRef)))
      (bind _output_get (Variables|Default|SetPlayerRef _asbp_third_person_character))))
  (if (and (Variables|/Game/ThirdPerson/Blueprints/BP_ThirdPersonCharacter.BP_ThirdPersonCharacter_C|GetbInteraction _output_get) (Variables|Default|GetbCanInteract))
    (CallFunction|AddtoInventory)))

(fn ConstructionScript)

(fn WidgetFacePlayer
  ;[0.15 0.15 0.15 0.5] Orient UI to Face Player
  (Transformation|SetWorldRotation (Variables|Default|GetPickUpMessage) (Math|Rotator|FindLookatRotation (Transformation|GetWorldLocation (Variables|Default|GetPickUpMessage)) (Transformation|GetWorldLocation (Variables|/Script/Engine.PlayerCameraManager|GetTransformComponent (Game|GetPlayerCameraManager 0)))) false false)
  (return))

(fn AddtoInventory
  ;[0.15 0.15 0.15 0.5] Check For Player
  (Utilities|IsValid (Variables|Default|GetPlayerRef)
    (:Is%20Valid
      _)
    (:Is%20Not%20Valid
      (bind _asbp_third_person_character (Utilities|Casting|CastToBP_ThirdPersonCharacter (Variables|Default|GetPlayerRef)))
      (bind _output_get (Variables|Default|SetPlayerRef _asbp_third_person_character))))
  ;[0.15 0.15 0.15 0.5] Increment Number of Health Items in Inventory
  (Variables|/Game/ThirdPerson/Blueprints/BP_Inventory.BP_Inventory_C|SetHealthItems (Variables|/Game/ThirdPerson/Blueprints/BP_ThirdPersonCharacter.BP_ThirdPersonCharacter_C|GetPlayerInventory _output_get) (+ (Variables|/Game/ThirdPerson/Blueprints/BP_Inventory.BP_Inventory_C|GetHealthItems (Variables|/Game/ThirdPerson/Blueprints/BP_ThirdPersonCharacter.BP_ThirdPersonCharacter_C|GetPlayerInventory _output_get)) 1))
  ;[0.15 0.15 0.15 0.5] Remove Collected Key From Map
  (Actor|DestroyActor self)
  (return))