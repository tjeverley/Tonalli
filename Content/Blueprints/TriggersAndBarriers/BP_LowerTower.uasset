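; Blueprint that lowers a tower actor once its referenced glyph puzzle is complete.
; Tick polls the puzzle's Complete flag and plays the LowerTower timeline until its finish sets Lowered.
; Each timeline update lerps the tower's current Z toward LoweredHeight, using the curve value divided by SpeedDampener as alpha, so movement compounds from the current position rather than a stored start.
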(event EventBeginPlay)

(event Collision|EventActorBeginOverlap
  (params (OtherActor :type Actor%20Object%20Reference)))

(event EventTick
  (params (DeltaSeconds :type Float%20%28single-precision%29))
  (bind _tower (Variables|Default|GetTower))
  (bind _returnvalue (Transformation|GetActorLocation _tower))
  (if (Variables|/Game/Blueprints/Puzzles/BP_GlyphPanel_8Buttons.BP_GlyphPanel_8Buttons_C|GetbComplete (Variables|Default|GetGlyphPuzzle))
    (if (not (Variables|Default|GetbLowered))
      (bind _lowerovertime (Timeline|LowerTower Play)
        (:Update
          (Transformation|SetActorLocation _tower (Math|Vector|MakeVector (.x _returnvalue) (.y _returnvalue) (Math|Float|Lerp (.z _returnvalue) (Variables|Default|GetLoweredHeight) (/ _lowerovertime (Variables|Default|GetSpeedDampener)))) false false))
        (:Finished
          (Variables|Default|SetbLowered true))))))

(fn ConstructionScript)