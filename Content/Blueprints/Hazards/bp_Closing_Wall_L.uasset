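; Closing wall hazard that slides along a configurable X, Y or Z axis and damages actors that overlap it.
; Tick starts that axis's Timeline when idle, lerping the Wall's relative location toward DistanceTravelled and clearing IsActive on finish.
; Each Timeline's Update feeds a Delay that triggers Reverse.
; Overlap applies small random damage, gated by a shared Hurt flag that resets shortly after overlap ends.
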(event Collision|EventActorBeginOverlap
  (params (OtherActor :type Actor%20Object%20Reference))
  ;[0.15 0.15 0.15 0.5] Applys Damage
  (if (not (Variables|Default|GetbHurt))
    (Game|Damage|ApplyDamage OtherActor (Math|Random|RandomFloatinRange 3.0 4.0) 0 0)
    (Variables|Default|SetbHurt true)))

(event EventTick
  (params (DeltaSeconds :type Float%20%28single-precision%29))
  (if (not (Variables|Default|GetbIsActive))
    (switch Utilities|FlowControl|Switch|SwitchonBP_EnumAxes (Variables|Default|GetDirection)
      (:NewEnumerator0
        ;[0.15 0.15 0.15 0.5] Moves on the X-Axis
        (Variables|Default|SetbIsActive true)
        (bind _newtrack_1 (Timeline|Timeline Play)
          (:Update
            (Transformation|SetRelativeLocation (Variables|Default|GetWall) (Math|Vector|MakeVector (Math|Float|Lerp 0.0 (Variables|Default|GetDistanceTravelled) _newtrack_1) 0.0 0.0) false false)
            (Utilities|FlowControl|Delay 3.0)
            (Timeline|Timeline Reverse))
          (:Finished
            (Variables|Default|SetbIsActive false))))
      (:NewEnumerator1
        ;[0.15 0.15 0.15 0.5] Moves on the Y-Axes
        (Variables|Default|SetbIsActive true)
        (bind _newtrack_1_2 (Timeline|Timeline_0 Play)
          (:Update
            (Transformation|SetRelativeLocation (Variables|Default|GetWall) (Math|Vector|MakeVector 0.0 (Math|Float|Lerp 0.0 (Variables|Default|GetDistanceTravelled) _newtrack_1_2) 0.0) false false)
            (Utilities|FlowControl|Delay 3.0)
            (Timeline|Timeline_0 Reverse))
          (:Finished
            (Variables|Default|SetbIsActive false))))
      (:NewEnumerator2
        ;[0.15 0.15 0.15 0.5] Moves on the Z-Axes
        (Variables|Default|SetbIsActive true)
        (bind _newtrack_1_3 (Timeline|Timeline_1 Play)
          (:Update
            (Transformation|SetRelativeLocation (Variables|Default|GetWall) (Math|Vector|MakeVector 0.0 0.0 (Math|Float|Lerp 0.0 (Variables|Default|GetDistanceTravelled) _newtrack_1_3)) false false)
            (Utilities|FlowControl|Delay 3.0)
            (Timeline|Timeline_1 Reverse))
          (:Finished
            (Variables|Default|SetbIsActive false)))))))

(event Collision|EventActorEndOverlap
  (params (OtherActor :type Actor%20Object%20Reference))
  ;[0.15 0.15 0.15 0.5] Applys Damage
  (Utilities|FlowControl|Delay 1.0)
  (Variables|Default|SetbHurt false))

(fn ConstructionScript)