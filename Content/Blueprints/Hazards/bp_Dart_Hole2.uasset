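; Dart hole hazard actor that repeatedly fires darts from its Arrow component.
; On Tick it spawns a Bp_Dart at the Arrow's transform, destroys it after BulletTime, then waits ShotDelay before firing again.
; The CanShoot flag acts as a busy lock despite its name: firing happens only while it is false, so one dart cycle runs at a time.
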(event EventBeginPlay)

(event Collision|EventActorBeginOverlap
  (params (OtherActor :type Actor%20Object%20Reference)))

(event EventTick
  (params (DeltaSeconds :type Float%20%28single-precision%29))
  (if (not (Variables|Default|GetbCanShoot))
    (bind _returnvalue (Game|SpawnActorfromClass "/Game/Blueprints/Hazards/bp_Dart.bp_Dart_C" (Transformation|GetWorldTransform (Variables|Default|Getarrow)) "AlwaysSpawn" "MultiplyWithRoot" 0 0))
    (Variables|Default|SetbCanShoot true)
    (Utilities|FlowControl|Delay (Variables|Default|GetBullet%20time))
    (Actor|DestroyActor _returnvalue)
    (Utilities|FlowControl|Delay (Variables|Default|GetShot%20delay))
    (Variables|Default|SetbCanShoot false)))

(fn ConstructionScript)