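; Dart trap hole hazard that automatically and repeatedly fires darts while its Override flag is off.
; Tick plays a 2D firing sound and spawns a Bp_Dart at the Arrow component's transform.
; Delays destroy the dart after BulletTime, then wait ShotDelay before the next shot.
; CanShoot acts as an inverted gate, set true during each firing cycle to block re-firing.
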(event EventBeginPlay)

(event Collision|EventActorBeginOverlap
  (params (OtherActor :type Actor%20Object%20Reference)))

(event EventTick
  (params (DeltaSeconds :type Float%20%28single-precision%29))
  (if (not (Variables|Default|GetbOverride))
    (if (not (Variables|Default|GetbCanShoot))
      (Audio|PlaySound2D "/Game/Audio/SoundEffects/HazardsAndEnemies/Fireing_Dart.Fireing_Dart" 1.0 1.0 0.0 0 0)
      (bind _returnvalue (Game|SpawnActorfromClass "/Game/Blueprints/Hazards/DartTrap/bp_Dart.bp_Dart_C" (Transformation|GetWorldTransform (Variables|Default|Getarrow)) "AlwaysSpawn" "MultiplyWithRoot" 0 0))
      (Variables|Default|SetbCanShoot true)
      (Utilities|FlowControl|Delay (Variables|Default|GetBulletTime))
      (Actor|DestroyActor _returnvalue)
      (Utilities|FlowControl|Delay (Variables|Default|GetShotDelay))
      (Variables|Default|SetbCanShoot false))))

(fn ConstructionScript)