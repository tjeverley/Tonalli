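; BP_JaguarFountain is a fountain actor that switches its Fountain component on or off based on the player's proximity.
; On BeginPlay it caches the player as BP_ThirdPersonCharacter.
; Every Tick it compares the distance to that player against ShutOffDistance, deactivating the fountain at or beyond it and activating it when closer, without resetting.
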(event EventBeginPlay
  (Utilities|IsValid (Variables|Default|GetPlayerRef)
    (:Is%20Not%20Valid
      (bind _asbp_third_person_character (Utilities|Casting|CastToBP_ThirdPersonCharacter (Game|GetPlayerCharacter 0)))
      (Variables|Default|SetPlayerRef _asbp_third_person_character))))

(event Collision|EventActorBeginOverlap
  (params (OtherActor :type Actor%20Object%20Reference)))

(event EventTick
  (params (DeltaSeconds :type Float%20%28single-precision%29))
  (bind _fountain (Variables|Default|GetFountain))
  (if (>= (Transformation|GetDistanceTo (Variables|Default|GetPlayerRef)) (Variables|Default|GetShutOffDistance))
    (Components|Activation|SetActive _fountain false false)
    (else
      (Components|Activation|SetActive _fountain true false))))

(fn ConstructionScript)