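; BP_FoundMessage is an interactable message actor that passes its name and contents to a dialogue box when the player interacts nearby.
; InteractionDetector overlaps cache the third-person character, toggle the prompt and CanInteract, and turn the prompt toward the camera on entry.
; Tick polls the player's Interaction flag and calls OpenMessage, which creates or reuses WBP_DialogueBox, pauses the game and shows the cursor.
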(event OnComponentBeginOverlap(InteractionDetector)
  (params (OverlappedComponent :type Primitive%20Component%20Object%20Reference) (OtherActor :type Actor%20Object%20Reference) (OtherComp :type Primitive%20Component%20Object%20Reference) (OtherBodyIndex :type Integer) (bFromSweep :type Boolean) (SweepResult :type Hit%20Result%20Structure%20%28by%20ref%29))
  ;[0.15 0.15 0.15 0.5] Display/Hide UI
  (Utilities|IsValid (Variables|Default|GetPlayerRef)
    (:Is%20Valid
      _)
    (:Is%20Not%20Valid
      (bind _asbp_third_person_character (Utilities|Casting|CastToBP_ThirdPersonCharacter OtherActor))
      (Variables|Default|SetPlayerRef _asbp_third_person_character)))
  (CallFunction|WidgetFacePlayer)
  (Rendering|SetVisibility (Variables|Default|GetInteractionMessage) true false)
  (Variables|Default|SetbCanInteract true))

(event OnComponentEndOverlap(InteractionDetector)
  (params (OverlappedComponent :type Primitive%20Component%20Object%20Reference) (OtherActor :type Actor%20Object%20Reference) (OtherComp :type Primitive%20Component%20Object%20Reference) (OtherBodyIndex :type Integer))
  ;[0.15 0.15 0.15 0.5] Display/Hide UI
  (Utilities|IsValid (Variables|Default|GetPlayerRef)
    (:Is%20Valid
      _)
    (:Is%20Not%20Valid
      (bind _asbp_third_person_character (Utilities|Casting|CastToBP_ThirdPersonCharacter OtherActor))
      (Variables|Default|SetPlayerRef _asbp_third_person_character)))
  (Rendering|SetVisibility (Variables|Default|GetInteractionMessage) false false)
  (Variables|Default|SetbCanInteract false))

(event EventBeginPlay
  ;[0.15 0.15 0.15 0.5] Default Values
  (Rendering|SetVisibility (Variables|Default|GetInteractionMessage) false false))

(event Collision|EventActorBeginOverlap
  (params (OtherActor :type Actor%20Object%20Reference)))

(event EventTick
  (params (DeltaSeconds :type Float%20%28single-precision%29))
  (Utilities|IsValid (Variables|Default|GetPlayerRef)
    (:Is%20Valid
      _)
    (:Is%20Not%20Valid
      (bind _asbp_third_person_character (Utilities|Casting|CastToBP_ThirdPersonCharacter (Variables|Default|GetPlayerRef)))
      (bind _output_get (Variables|Default|SetPlayerRef _asbp_third_person_character))))
  (if (and (Variables|/Game/ThirdPerson/Blueprints/BP_ThirdPersonCharacter.BP_ThirdPersonCharacter_C|GetbInteraction _output_get) (Variables|Default|GetbCanInteract))
    (CallFunction|OpenMessage)))

(fn ConstructionScript)

(fn WidgetFacePlayer
  ;[0.15 0.15 0.15 0.5] Orient UI To Face Player
  (Transformation|SetWorldRotation (Variables|Default|GetInteractionMessage) (Math|Rotator|FindLookatRotation (Transformation|GetWorldLocation (Variables|Default|GetInteractionMessage)) (Transformation|GetWorldLocation (Variables|/Script/Engine.PlayerCameraManager|GetTransformComponent (Game|GetPlayerCameraManager 0)))) false false)
  (return))

(fn OpenMessage
  (bind _returnvalue (Game|GetPlayerController 0))
  (Utilities|IsValid (Variables|Default|GetMessageRef)
    (:Is%20Valid
      _)
    (:Is%20Not%20Valid
      (bind _returnvalue_2 (UserInterface|CreateWidget "/Game/UI/HUD/WBP_DialogueBox.WBP_DialogueBox_C" _returnvalue))
      (bind _output_get (Variables|Default|SetMessageRef _returnvalue_2))))
  (Variables|/Game/UI/HUD/WBP_DialogueBox.WBP_DialogueBox_C|SetNameVar _output_get (Variables|Default|GetMessageName))
  (Variables|/Game/UI/HUD/WBP_DialogueBox.WBP_DialogueBox_C|SetDialogueVar _output_get (Variables|Default|GetMessageContents))
  (Game|SetGamePaused true)
  (Input|SetInputModeGameandUI _returnvalue 0 "DoNotLock" false false)
  (Variables|/Script/Engine.PlayerController|SetbShowMouseCursor _returnvalue true)
  (return))