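; Behavior tree task for the Stone Ranged Golem, named for retreating, that sets the golem's walk speed.
; On AI execution it casts the controlled pawn to BP_StoneRangedGolem, applies its MaxWalkSpeed variable to CharacterMovement and finishes successfully.
; It issues no movement itself, and a failed cast never finishes the task.
; The branch is always true, as the player-too-close comparison is leftover logic that never runs.
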(event EventReceiveExecuteAI
  (params (OwnerController :type AI%20Controller%20Object%20Reference) (ControlledPawn :type Pawn%20Object%20Reference))
  ;[0.15 0.15 0.15 0.5] Walk Speed Logic
  (if true
    (bind _asbp_stone_ranged_golem (Utilities|Casting|CastToBP_StoneRangedGolem ControlledPawn))
    (Variables|/Script/Engine.CharacterMovementComponent|SetMaxWalkSpeed (Variables|/Script/Engine.Character|GetCharacterMovement _asbp_stone_ranged_golem) (Variables|Default|GetMaxWalkSpeed))
    (AI|BehaviorTree|FinishExecute true)))