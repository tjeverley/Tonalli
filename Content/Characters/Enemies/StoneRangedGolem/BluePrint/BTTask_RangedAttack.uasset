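; Behavior tree task that performs the stone ranged golem's dart attack on the player.
; It sets the golem's attacking flag, plays the ranged attack animation directly on the mesh and turns it once to face the player.
; After a delay it spawns a dart at the shot point, destroys it after another delay, then clears the flag and finishes successfully.
; A failed pawn cast only prints a message and never finishes the task.
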(event EventReceiveExecuteAI
  (params (OwnerController :type AI%20Controller%20Object%20Reference) (ControlledPawn :type Pawn%20Object%20Reference))
  (bind _asbp_stone_ranged_golem (Utilities|Casting|CastToBP_StoneRangedGolem ControlledPawn)
    (:then
      (Variables|/Game/Characters/Enemies/StoneRangedGolem/BluePrint/BP_StoneRangedGolem.BP_StoneRangedGolem_C|SetbIsAttacking _asbp_stone_ranged_golem true)
      (Components|Animation|PlayAnimation (Variables|/Script/Engine.Character|GetMesh _asbp_stone_ranged_golem) "/Game/Characters/Enemies/StoneRangedGolem/RangedAnimation/GolemAttack_Ranged_Anim.GolemAttack_Ranged_Anim" false)
      (Transformation|SetActorRotation _asbp_stone_ranged_golem (Math|Rotator|FindLookatRotation (Transformation|GetActorLocation _asbp_stone_ranged_golem) (Transformation|GetActorLocation (Game|GetPlayerCharacter 0))))
      (Development|PrintString (Utilities|String|ToString(Rotator) (Math|Rotator|FindLookatRotation (Transformation|GetActorLocation _asbp_stone_ranged_golem) (Transformation|GetActorLocation (Game|GetPlayerCharacter 0)))))
      (Utilities|FlowControl|Delay 3.0)
      (bind _returnvalue (Game|SpawnActorfromClass "/Game/Blueprints/Hazards/bp_Dart.bp_Dart_C" (Math|Transform|MakeTransform (.location (Transformation|GetWorldTransform (Variables|/Game/Characters/Enemies/StoneRangedGolem/BluePrint/BP_StoneRangedGolem.BP_StoneRangedGolem_C|GetShot%20Point _asbp_stone_ranged_golem))) (.rotation (Transformation|GetWorldTransform (Variables|/Game/Characters/Enemies/StoneRangedGolem/BluePrint/BP_StoneRangedGolem.BP_StoneRangedGolem_C|GetShot%20Point _asbp_stone_ranged_golem))) "1.000000,1.000000,1.000000") "AlwaysSpawn" "MultiplyWithRoot" 0 0))
      (Utilities|FlowControl|Delay 2.0)
      (Actor|DestroyActor _returnvalue)
      (Variables|/Game/Characters/Enemies/StoneRangedGolem/BluePrint/BP_StoneRangedGolem.BP_StoneRangedGolem_C|SetbIsAttacking _asbp_stone_ranged_golem false)
      (AI|BehaviorTree|FinishExecute true))
    (:CastFailed
      (Development|PrintString "attack fai;"))))