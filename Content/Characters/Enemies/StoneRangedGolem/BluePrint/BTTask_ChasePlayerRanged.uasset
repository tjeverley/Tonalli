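; Behavior Tree task that makes the ranged stone golem chase the player.
; Each execution writes the player's location to the PlayerLocationVector blackboard key and, unless the golem is attacking, issues a move that stops at a standoff radius.
; It finishes successfully at once without waiting for the move to complete.
; Unconnected leftover nodes for rotation, attack animation and dart spawning never run.
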(event EventReceiveExecuteAI
  (params (OwnerController :type AI%20Controller%20Object%20Reference) (ControlledPawn :type Pawn%20Object%20Reference))
  (bind _returnvalue (Game|GetPlayerCharacter 0))
  (bind _returnvalue_2 (Transformation|GetActorLocation _returnvalue))
  (bind _asbp_stone_ranged_golem (Utilities|Casting|CastToBP_StoneRangedGolem ControlledPawn))
  ;[0.15 0.15 0.15 0.5] Chase Logic
  (if (Variables|/Game/Characters/Enemies/StoneRangedGolem/BluePrint/BP_StoneRangedGolem.BP_StoneRangedGolem_C|GetbIsAttacking _asbp_stone_ranged_golem)
    (AI|BehaviorTree|SetBlackboardValueasVector (Variables|Default|GetPlayer%20Location%20Vector) (Transformation|GetActorLocation (Game|GetPlayerCharacter 0)))
    (else
      (AI|BehaviorTree|SetBlackboardValueasVector (Variables|Default|GetPlayer%20Location%20Vector) _returnvalue_2)
      (AI|Navigation|MovetoLocation OwnerController _returnvalue_2 4e+02 true true false true 0)))
  (AI|BehaviorTree|FinishExecute true))