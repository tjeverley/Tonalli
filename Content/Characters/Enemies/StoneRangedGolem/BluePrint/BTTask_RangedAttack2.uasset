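; Behavior tree task that runs the stone ranged golem's dart attack.
; On execute it flags the golem as attacking, plays the ranged attack animation, then after a delay plays a firing sound and spawns a dart at the ShotPoint transform.
; After a further delay it destroys the dart, clears the flag and finishes successfully.
; While ticking, it yaws the golem to face the player, keeping its own height for a level look-at.
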(event EventReceiveExecuteAI
  (params (OwnerController :type AI%20Controller%20Object%20Reference) (ControlledPawn :type Pawn%20Object%20Reference))
  (bind _asbp_stone_ranged_golem (Utilities|Casting|CastToBP_StoneRangedGolem ControlledPawn))
  ;[0.15 0.15 0.15 0.5] Attacks
  (Variables|/Game/Characters/Enemies/StoneRangedGolem/BluePrint/BP_StoneRangedGolem.BP_StoneRangedGolem_C|SetbIsAttacking _asbp_stone_ranged_golem true)
  (Components|Animation|PlayAnimation (Variables|/Script/Engine.Character|GetMesh _asbp_stone_ranged_golem) "/Game/Characters/Enemies/StoneRangedGolem/RangedAnimation/GolemAttack_Ranged_Anim.GolemAttack_Ranged_Anim" false)
  (Utilities|FlowControl|Delay 3.0)
  (Audio|PlaySound2D "/Game/Audio/SoundEffects/HazardsAndEnemies/Fireing_Dart.Fireing_Dart" 1.0 1.0 0.0 0 0)
  (bind _returnvalue (Game|SpawnActorfromClass "/Game/Blueprints/Hazards/DartTrap/bp_Dart.bp_Dart_C" (Math|Transform|MakeTransform (.location (Transformation|GetWorldTransform (Variables|/Game/Characters/Enemies/StoneRangedGolem/BluePrint/BP_StoneRangedGolem.BP_StoneRangedGolem_C|GetShot%20Point _asbp_stone_ranged_golem))) (.rotation (Transformation|GetWorldTransform (Variables|/Game/Characters/Enemies/StoneRangedGolem/BluePrint/BP_StoneRangedGolem.BP_StoneRangedGolem_C|GetShot%20Point _asbp_stone_ranged_golem))) "1.000000,1.000000,1.000000") "AlwaysSpawn" "MultiplyWithRoot" 0 0))
  (Utilities|FlowControl|Delay 2.0)
  (Actor|DestroyActor _returnvalue)
  (Variables|/Game/Characters/Enemies/StoneRangedGolem/BluePrint/BP_StoneRangedGolem.BP_StoneRangedGolem_C|SetbIsAttacking _asbp_stone_ranged_golem false)
  (AI|BehaviorTree|FinishExecute true))

(event EventReceiveTickAI
  (params (OwnerController :type AI%20Controller%20Object%20Reference) (ControlledPawn :type Pawn%20Object%20Reference) (DeltaSeconds :type Float%20%28single-precision%29))
  (bind _returnvalue (Game|GetPlayerCharacter 0))
  (bind _returnvalue_2 (Transformation|GetActorLocation _returnvalue))
  ;[0.15 0.15 0.15 0.5] Looks at the player
  (Transformation|SetActorRotation ControlledPawn (Math|Rotator|FindLookatRotation (Math|Vector|MakeVector (.x (Transformation|GetActorLocation (stale EventReceiveExecuteAI _asbp_stone_ranged_golem))) (.y (Transformation|GetActorLocation (stale EventReceiveExecuteAI _asbp_stone_ranged_golem))) (.z (Transformation|GetActorLocation (stale EventReceiveExecuteAI _asbp_stone_ranged_golem)))) (Math|Vector|MakeVector (.x _returnvalue_2) (.y _returnvalue_2) (.z (Transformation|GetActorLocation (stale EventReceiveExecuteAI _asbp_stone_ranged_golem)))))))