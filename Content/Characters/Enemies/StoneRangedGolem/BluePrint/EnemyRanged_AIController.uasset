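; AI controller for the ranged Stone Golem enemy, which runs the BT_AI_EnemyRanged behavior tree on BeginPlay.
; Perception updates for actors tagged "Enemy" write the sensed state to the bCanSeePlayer blackboard key.
; Tick sets bInAttackDistance by checking the controlled pawn's distance to the first player character against a fixed threshold.
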(event OnTargetPerceptionUpdated(AIPerception)
  (params (Actor :type Actor%20Object%20Reference) (Stimulus :type AI%20Stimulus%20Structure))
  ;[0.15 0.15 0.15 0.5] Sight Perception Logic
  (if (Actor|ActorHasTag Actor "Enemy")
    (AI|Components|Blackboard|SetValueasBool (AI|GetBlackboard 0) (Utilities|Name|MakeLiteralName "bCanSeePlayer") (.bSuccessfullySensed (Utilities|Struct|BreakAIStimulus Stimulus)))))

(event EventBeginPlay
  ;[0.15 0.15 0.15 0.5] Runs Behaviour Tree
  (AI|RunBehaviorTree "/Game/Characters/Enemies/StoneRangedGolem/BluePrint/BT_AI_EnemyRanged.BT_AI_EnemyRanged"))

(event EventTick
  (params (DeltaSeconds :type Float%20%28single-precision%29))
  ;[0.15 0.15 0.15 0.5] Logic for the attack distance
  (AI|Components|Blackboard|SetValueasBool (AI|GetBlackboard 0) (Utilities|Name|MakeLiteralName "bInAttackDistance") (<= (Transformation|GetDistanceTo (Pawn|GetControlledPawn) (Game|GetPlayerCharacter 0)) 6e+02)))

(fn ConstructionScript)