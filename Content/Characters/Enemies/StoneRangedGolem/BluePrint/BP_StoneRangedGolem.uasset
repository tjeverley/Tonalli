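; BP_StoneRangedGolem is a ranged stone golem enemy Blueprint with health and a death effect; its attack event is still empty.
; Collision overlap caches the third-person player and sets a timer for LoopAttacking, which end overlap re-sets without a specified time.
; Any damage lowers GolemHealth.
; Tick polls health and, at zero or below, hides the mesh, activates the despawn burst and destroys the actor after a delay.
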(event OnComponentBeginOverlap(collision)
  (params (OverlappedComponent :type Primitive%20Component%20Object%20Reference) (OtherActor :type Actor%20Object%20Reference) (OtherComp :type Primitive%20Component%20Object%20Reference) (OtherBodyIndex :type Integer) (bFromSweep :type Boolean) (SweepResult :type Hit%20Result%20Structure%20%28by%20ref%29))
  (Utilities|IsValid (Variables|Default|GetPlayer%20Ref)
    (:Is%20Valid
      _)
    (:Is%20Not%20Valid
      (bind _asbp_third_person_character (Utilities|Casting|CastToBP_ThirdPersonCharacter OtherActor))
      (Variables|Default|SetPlayer%20Ref _asbp_third_person_character)))
  (Utilities|Time|SetTimerbyEvent (delegate Custom|LoopAttacking) 1.2))

(event OnComponentEndOverlap(collision)
  (params (OverlappedComponent :type Primitive%20Component%20Object%20Reference) (OtherActor :type Actor%20Object%20Reference) (OtherComp :type Primitive%20Component%20Object%20Reference) (OtherBodyIndex :type Integer))
  (Utilities|Time|SetTimerbyEvent (delegate Custom|LoopAttacking) 0.0))

(event Custom|LoopAttacking)

(event EventBeginPlay)

(event Collision|EventActorBeginOverlap
  (params (OtherActor :type Actor%20Object%20Reference)))

(event EventTick
  (params (DeltaSeconds :type Float%20%28single-precision%29))
  ;[0.15 0.15 0.15 0.5] Death
  (if (<= (Variables|Default|GetGolemHealth) 0.0)
    (Rendering|SetVisibility (Variables|Character|GetMesh) false false)
    (Components|Activation|SetActive (Variables|Default|GetFX_DespawnBurst) true false)
    (Utilities|FlowControl|Delay 2.0)
    (Actor|DestroyActor)))

(event Game|Damage|EventAnyDamage
  (params (Damage :type Float%20%28single-precision%29) (DamageType :type Damage%20Type%20Object%20Reference) (InstigatedBy :type Controller%20Object%20Reference) (DamageCauser :type Actor%20Object%20Reference))
  ;[0.15 0.15 0.15 0.5] Take Damage
  (Variables|Default|SetGolemHealth (- (Variables|Default|GetGolemHealth) Damage)))

(fn ConstructionScript)