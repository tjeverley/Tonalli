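; Stone melee golem enemy that punches the player and can be killed.
; Entering its Collision volume caches the player and sets a timer for the attack animation, and leaving resets that timer with no delay, clearing it.
; The attack briefly raises a Punch flag that lets PunchCollider overlaps damage the cached player.
; Incoming damage lowers health, and Tick handles death by hiding the mesh, activating a despawn burst and destroying the actor after a delay.
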(event OnComponentBeginOverlap(PunchCollider)
  (params (OverlappedComponent :type Primitive%20Component%20Object%20Reference) (OtherActor :type Actor%20Object%20Reference) (OtherComp :type Primitive%20Component%20Object%20Reference) (OtherBodyIndex :type Integer) (bFromSweep :type Boolean) (SweepResult :type Hit%20Result%20Structure%20%28by%20ref%29))
  ;[0.15 0.15 0.15 0.5] Damage Player
  (if (Variables|Default|GetbPunch)
    (Utilities|IsValid (Variables|Default|GetPlayerRef)
      (:Is%20Valid
        _)
      (:Is%20Not%20Valid
        (bind _asbp_third_person_character (Utilities|Casting|CastToBP_ThirdPersonCharacter OtherActor))
        (bind _output_get (Variables|Default|SetPlayerRef _asbp_third_person_character))))
    (Game|Damage|ApplyDamage _output_get 15.0 0 self)))

(event OnComponentEndOverlap(Collision)
  (params (OverlappedComponent :type Primitive%20Component%20Object%20Reference) (OtherActor :type Actor%20Object%20Reference) (OtherComp :type Primitive%20Component%20Object%20Reference) (OtherBodyIndex :type Integer))
  ;[0.15 0.15 0.15 0.5] Attack Behaviour
  (Utilities|Time|SetTimerbyEvent (delegate Custom|LoopAttacking) 0.0))

(event OnComponentBeginOverlap(Collision)
  (params (OverlappedComponent :type Primitive%20Component%20Object%20Reference) (OtherActor :type Actor%20Object%20Reference) (OtherComp :type Primitive%20Component%20Object%20Reference) (OtherBodyIndex :type Integer) (bFromSweep :type Boolean) (SweepResult :type Hit%20Result%20Structure%20%28by%20ref%29))
  ;[0.15 0.15 0.15 0.5] Attack Behaviour
  (Utilities|IsValid (Variables|Default|GetPlayerRef)
    (:Is%20Valid
      _)
    (:Is%20Not%20Valid
      (bind _asbp_third_person_character (Utilities|Casting|CastToBP_ThirdPersonCharacter OtherActor))
      (Variables|Default|SetPlayerRef _asbp_third_person_character)))
  (Utilities|Time|SetTimerbyEvent (delegate Custom|LoopAttacking) 1.2))

(event Custom|LoopAttacking
  ;[0.15 0.15 0.15 0.5] Attack Behaviour
  (Utilities|FlowControl|Sequence
    (:then_0
      (Components|Animation|PlayAnimation (Variables|Character|GetMesh) "/Game/Characters/Enemies/StoneMeleeGolom/Animations/Animation/GolemAttack_REEXPORT_Anim.GolemAttack_REEXPORT_Anim" false))
    (:then_1
      (Variables|Default|SetbPunch true)
      (Utilities|FlowControl|Delay 0.1)
      (Variables|Default|SetbPunch false))))

(event EventBeginPlay)

(event Collision|EventActorBeginOverlap
  (params (OtherActor :type Actor%20Object%20Reference)))

(event EventTick
  (params (DeltaSeconds :type Float%20%28single-precision%29))
  ;[0.15 0.15 0.15 0.5] Death
  (if (<= (Variables|Default|GetGolemHealth) 0.0)
    (Rendering|SetVisibility (Variables|Character|GetMesh) false false)
    (Components|Activation|SetActive (Variables|Default|GetFX_DespawnBurst) true false)
    (Utilities|FlowControl|Delay 2.0)
    (Actor|DestroyActor)))

(event Game|Damage|EventAnyDamage
  (params (Damage :type Float%20%28single-precision%29) (DamageType :type Damage%20Type%20Object%20Reference) (InstigatedBy :type Controller%20Object%20Reference) (DamageCauser :type Actor%20Object%20Reference))
  ;[0.15 0.15 0.15 0.5] Take Damage
  (Variables|Default|SetGolemHealth (- (Variables|Default|GetGolemHealth) Damage)))

(fn ConstructionScript)